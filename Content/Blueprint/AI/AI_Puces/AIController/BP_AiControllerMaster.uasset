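; Base AI controller for the Puces enemies, running a behavior tree that drives patrol and investigation.
; On BeginPlay it seeds the blackboard from the pawn's patrol path.
; Perception updates dispatch by sense class: sight tracks the player and reports alert levels to the character, while hearing stores the noise location.
; Events halt the tree for timed paralysis or montage-backed stun, or set a search location for a Puce killer.
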(event `self.ReceiveBeginPlay`
  (`self.RunBehaviorTree` (`self.BTAsset`))
  (bind _asbp_ai_master (cast `/Game/Blueprint/AI/AI_Puces/AiCharacter/BP_AI_Master` (`self.K2_GetPawn`)))
  (bind _output_get (set `self.As BP AI Master` _asbp_ai_master))
  (`BlackboardComponent.SetValueAsBool` (`AIBlueprintHelperLibrary.GetBlackboard` null) "PathLooping" (`/Game/Blueprint/AI/BP_PatrolPath.IsLooping` (`/Game/Blueprint/AI/AI_Puces/AiCharacter/BP_AI_Master.PatrolPath` _output_get)))
  (`BlackboardComponent.SetValueAsInt` (`AIBlueprintHelperLibrary.GetBlackboard` null) "Direction" 1)
  (`BlackboardComponent.SetValueAsFloat` (`AIBlueprintHelperLibrary.GetBlackboard` null) "WaitTime" (`/Game/Blueprint/AI/BP_PatrolPath.WaitTime` (`/Game/Blueprint/AI/AI_Puces/AiCharacter/BP_AI_Master.PatrolPath` (`self.As BP AI Master`)))))

(event `self.AIPerception.OnTargetPerceptionUpdated`
  (params (Actor :type "Actor Object Reference") (Stimulus :type "AIStimulus Structure"))
  (bind _returnvalue (`AIPerceptionSystem.GetSenseClassForStimulus` Stimulus))
  (`self.HandleSense` (`KismetSystemLibrary.GetClassDisplayName` _returnvalue) Actor Stimulus))

(event `Paralysed`
  (params (ParalysedTime :type "Float (double-precision)") (`Behavior tree` :type "BehaviorTree Object Reference"))
  (`BlackboardComponent.SetValueAsBool` (`AIBlueprintHelperLibrary.GetBlackboard` null) "IsInvestigating?" false)
  (`self.StopMovement`)
  (`BrainComponent.StopLogic` (`self.BrainComponent`) "")
  (`KismetSystemLibrary.Delay` ParalysedTime)
  (`self.RunBehaviorTree` `Behavior tree`))

(event `Stunned`
  (params (StunnedTime :type "Float (double-precision)"))
  (`self.StopMovement`)
  (`BrainComponent.StopLogic` (`self.BrainComponent`) "")
  (`|PlayMontage` null
    (:`then`
      (`KismetSystemLibrary.Delay` StunnedTime)
      (`BrainComponent.RestartLogic` (`self.BrainComponent`)))))

(event `SearchPuceKiller`
  (params (Vector3 :type "Vector Structure"))
  (`BlackboardComponent.SetValueAsVector` (`self.Blackboard`) "TargetLocationVector" Vector3))

(fn `HandleSense`
  (params (Selection :type String) (SensedActor :type "Actor Object Reference") (Stimulus :type "AIStimulus Structure"))
  (bind ((`bSuccessfullySensed` _bsuccessfullysensed)) (break `AIStimulus` (`local.Stimulus`)))
  (switch `string` Selection
    (:`AISense_Sight`
      ;[0 0 1] Sight
      (if (`self.ActorHasTag` (`local.SensedActor`) "Player")
        (`BlackboardComponent.SetValueAsBool` (`self.Blackboard`) "IsInvestigating?" _bsuccessfullysensed)
        (if _bsuccessfullysensed
          (if (`self.ActorHasTag` (`local.SensedActor`) "Player")
            (`BlackboardComponent.SetValueAsObject` (`self.Blackboard`) "TargetLocationActor" (`local.SensedActor`))
            (bind _ascharacter_master (cast `/Game/Blueprint/Character/CharacterMaster` (`local.SensedActor`)))
            (`/Game/Blueprint/Character/CharacterMaster.NewAlertState` _ascharacter_master self 2))
          (else
            (`BlackboardComponent.SetValueAsVector` (`self.Blackboard`) "TargetLocationVector" (`.StimulusLocation` (break `AIStimulus` (`local.Stimulus`))))
            (`BlackboardComponent.SetValueAsObject` (`self.Blackboard`) "TargetLocationActor" null)
            (bind _ascharacter_master_2 (cast `/Game/Blueprint/Character/CharacterMaster` (`local.SensedActor`)))
            (`/Game/Blueprint/Character/CharacterMaster.NewAlertState` _ascharacter_master_2 self 1)))))
    (:`AISense_Hearing`
      ;[-0 0 1] Hearing
      (`BlackboardComponent.SetValueAsBool` (`self.Blackboard`) "IsInvestigating?" (`.bSuccessfullySensed` (break `AIStimulus` (`local.Stimulus`))))
      (`BlackboardComponent.SetValueAsVector` (`self.Blackboard`) "TargetLocationVector" (`.StimulusLocation` (break `AIStimulus` (`local.Stimulus`)))))))

(fn `UserConstructionScript`)