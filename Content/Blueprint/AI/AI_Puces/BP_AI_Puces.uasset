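; BP_AI_Puces is an AI character with an alert state and health.
; ChangeState stores the new state and sets walk speed for Neutral, Investigate or Alert through a DoOnce, which ResetAlert re-arms immediately afterwards.
; TakeDamage subtracts from Health, prints the remaining value and destroys the actor at zero or below.
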(event `/Game/Blueprint/AI/AI_Puces/BPI_ChangeAiStates.ChangeState`
  (params (AlertState :type "/Game/Blueprint/AI/AI_Puces/E_AIStates Enum" :default "NewEnumerator1"))
  (set `self.Alert State` AlertState)
  (`/Engine/EditorBlueprintResources/StandardMacros.DoOnce` false :!label _label
    (:`Completed`
      (set `CharacterMovementComponent.MaxWalkSpeed` (select `/Game/Blueprint/AI/AI_Puces/E_AIStates` (`self.Alert State`) :`NewEnumerator1` 350.0 :`NewEnumerator2` 400.0 :`NewEnumerator3` 500.0 :!type "Float (single-precision)") (`self.CharacterMovement`))
      (`self.ResetAlert`))))

(event `ResetAlert`
  (goto _label :!via `Reset`))

(event `/Game/Blueprint/BPI_Damageable.TakeDamage`
  (params (Damage :type "Float (single-precision)"))
  (bind _output_get (set `self.Health` (- (`self.Health`) Damage)))
  (`KismetSystemLibrary.PrintString` (`KismetStringLibrary.Conv_DoubleToString` _output_get))
  (if (<= (`self.Health`) 0.0)
    (`self.K2_DestroyActor`)))

(fn `UserConstructionScript`)