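; AI controller for the Puces enemy that runs its behavior tree and feeds perception results into the Blackboard.
; Sight sets the player as target actor, or on loss stores the last stimulus location and clears the actor.
; Hearing stores the noise location, and both senses drive the investigating flag.
; A BP_RelaySound event toggles the melee loudness between full and half through a FlipFlop.
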(event `self.ReceiveBeginPlay`
  (`self.RunBehaviorTree` "/Game/Blueprint/AI/AI_Puces/BT_EnnemyPuces.BT_EnnemyPuces")
  (bind _returnvalue (`GameplayStatics.GetActorOfClass` "/Game/Blueprint/WorldMechanics/Relay/BP_RelaySound.BP_RelaySound_C"))
  (`/Engine/EditorBlueprintResources/StandardMacros.IsValid` _returnvalue
    (:`Is Valid`
      (add `/Game/Blueprint/WorldMechanics/Relay/BP_RelaySound.RiseAiMeleeAttackLoudness` _returnvalue (delegate `RiseMeleeLoudness`)))))

(event `RiseMeleeLoudness`
  (`/Engine/EditorBlueprintResources/StandardMacros.FlipFlop`
    (:`A`
      (set `self.MeleeLoudness` 1.0))
    (:`B`
      (set `self.MeleeLoudness` 0.5))))

(event `self.AIPerception.OnTargetPerceptionUpdated`
  (params (Actor :type "Actor Object Reference") (Stimulus :type "AIStimulus Structure"))
  (bind ((`bSuccessfullySensed` _bsuccessfullysensed)) (break `AIStimulus` Stimulus))
  (bind _returnvalue (`AIPerceptionSystem.GetSenseClassForStimulus` Stimulus))
  (switch `string` (`KismetSystemLibrary.GetClassDisplayName` _returnvalue)
    (:`AISense_Sight`
      (`BlackboardComponent.SetValueAsBool` (`self.Blackboard`) "IsInvestigating?" _bsuccessfullysensed)
      (if _bsuccessfullysensed
        (if (== Actor (`GameplayStatics.GetPlayerCharacter` 0))
          (`BlackboardComponent.SetValueAsObject` (`self.Blackboard`) "TargetLocationActor" Actor))
        (else
          (`BlackboardComponent.SetValueAsVector` (`self.Blackboard`) "TargetLocationVector" (`.StimulusLocation` (break `AIStimulus` Stimulus)))
          (`BlackboardComponent.SetValueAsObject` (`self.Blackboard`) "TargetLocationActor" null))))
    (:`AISense_Hearing`
      (`BlackboardComponent.SetValueAsBool` (`self.Blackboard`) "IsInvestigating?" (`.bSuccessfullySensed` (break `AIStimulus` Stimulus)))
      (`BlackboardComponent.SetValueAsVector` (`self.Blackboard`) "TargetLocationVector" (`.StimulusLocation` (break `AIStimulus` Stimulus))))))

(fn `UserConstructionScript`)