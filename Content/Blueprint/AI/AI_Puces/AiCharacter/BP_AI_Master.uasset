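; Base AI character for the Puce enemies, handling alert states, health and death.
; ChangeState maps Neutral, Investigate and Alert to walk speed and to detected or search widgets, through a DoOnce that immediately resets.
; Lethal damage resets the player's alert UI for this AI's controller, spawns a dead body and destroys the actor.
; A retriggerable delay hides the custom-depth outline and Niagara trace.
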(event `self.ReceiveBeginPlay`
  (bind _foundwidgets (`WidgetBlueprintLibrary.GetAllWidgetsOfClass` "/Game/UI/UI_InGame/Widget_HeadUp.Widget_HeadUp_C" false))
  (set `self.W_HeadUpRef` (`|GetArrayItem` _foundwidgets))
  (bind _ascharacter_master (cast `/Game/Blueprint/Character/CharacterMaster` (`GameplayStatics.GetPlayerCharacter` 0)))
  (set `self.As Character Master` _ascharacter_master)
  (bind _asbp_ai_controller_master (cast `/Game/Blueprint/AI/AI_Puces/AIController/BP_AiControllerMaster` (`AIBlueprintHelperLibrary.GetAIController` self)))
  (set `self.As BP Ai Controller Master` _asbp_ai_controller_master))

(event `/Game/Blueprint/AI/AI_Puces/BPI_ChangeAiStates.ChangeState`
  (params (AlertState :type "/Game/Blueprint/AI/AI_Puces/E_AIStates Enum" :default "NewEnumerator1"))
  (set `self.Alert State` AlertState)
  (`/Engine/EditorBlueprintResources/StandardMacros.DoOnce` false :!label _label
    (:`Completed`
      (set `CharacterMovementComponent.MaxWalkSpeed` (select `/Game/Blueprint/AI/AI_Puces/E_AIStates` (`self.Alert State`) :`NewEnumerator1` 350.0 :`NewEnumerator2` 400.0 :`NewEnumerator3` 500.0 :!type "Float (single-precision)") (`self.CharacterMovement`))
      (switch `/Game/Blueprint/AI/AI_Puces/E_AIStates` (`self.Alert State`)
        (:`NewEnumerator1`
          (`self.SetWidgetVisibility` false))
        (:`NewEnumerator2`
          (`self.SetWidgetVisibility` false true))
        (:`NewEnumerator3`
          (`self.SetWidgetVisibility` true)))
      (`self.ResetAlert`))))

(event `ResetAlert`
  (goto _label :!via `Reset`))

(event `/Game/Blueprint/BPI_Damageable.TakeDamage`
  (params (Damage :type "Float (single-precision)"))
  (`self.AiTakeDamage` Damage))

(event `HIdeOutlineAndVFX`
  (`KismetSystemLibrary.RetriggerableDelay` 10.0)
  (`SceneComponent.SetHiddenInGame` (`self.NS_TempoPuceTrace`) true false)
  (`PrimitiveComponent.SetRenderCustomDepth` (`self.Mesh`) false))

(fn `AiTakeDamage`
  (params (DamageTaken :type "Float (double-precision)"))
  (bind _output_get (set `self.Health` (- (`self.Health`) DamageTaken)))
  (`KismetSystemLibrary.PrintString` (`KismetStringLibrary.Conv_DoubleToString` _output_get))
  (if (<= (`self.Health`) 0.0)
    (`/Game/Blueprint/Character/CharacterMaster.ResetAlertLevelUI` (`self.As Character Master`) (`self.As BP Ai Controller Master`))
    (`|SpawnActorFromClass` "/Game/Blueprint/Actors/DeadBody/BP_PuceDeadBody.BP_PuceDeadBody_C" (`self.GetTransform` self) "Undefined" "OverrideRootScale" null null)
    (`self.K2_DestroyActor`)))

(fn `UserConstructionScript`)