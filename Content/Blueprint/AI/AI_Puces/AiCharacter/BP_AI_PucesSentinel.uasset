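; Sentinel "Puce" AI enemy that latches onto a player character on sphere overlap and acts as a noise beacon.
; An attack switches control to the victim if needed, starts NewPuceAttack, attaches to a random mesh socket, unpossesses and slows nearby characters.
; It repeatedly reports noise, with loudness toggled by BP_RelaySound, until QTeIsComplete restores the player and destroys it.
; Its own button-mash QTE logic is disconnected.
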(event `self.ReceiveBeginPlay`
  (`parent.ReceiveBeginPlay`)
  (bind _returnvalue (`GameplayStatics.GetActorOfClass` "/Game/Blueprint/WorldMechanics/Relay/BP_RelaySound.BP_RelaySound_C"))
  (`/Engine/EditorBlueprintResources/StandardMacros.IsValid` _returnvalue
    (:`Is Valid`
      (add `/Game/Blueprint/WorldMechanics/Relay/BP_RelaySound.RiseAiMeleeAttackLoudness` _returnvalue (delegate `RiseMeleeLoudness`)))
    (:`Is Not Valid`
      _))
  (bind _asbp_ai_controller_master (cast `/Game/Blueprint/AI/AI_Puces/AIController/BP_AiControllerMaster` (`AIBlueprintHelperLibrary.GetAIController` self)))
  (set `self.As BP Ai Controller Master_0` _asbp_ai_controller_master))

(event `RiseMeleeLoudness`
  (`/Engine/EditorBlueprintResources/StandardMacros.FlipFlop`
    (:`A`
      (set `self.MeleeLoudness` 1.0))
    (:`B`
      (set `self.MeleeLoudness` 0.5))))

(event `/Game/Blueprint/AI/AI_Puces/BPI_ChangeAiStates.ChangeState`
  (params (AlertState :type "/Game/Blueprint/AI/AI_Puces/E_AIStates Enum" :default "NewEnumerator1"))
  (`parent.ChangeState` AlertState))

(event `/Game/Blueprint/BPI_Damageable.TakeDamage`
  (params (Damage :type "Float (single-precision)"))
  (`parent.TakeDamage` Damage))

(event `ContinueMeleeAttack`
  (bind _returnvalue (`self.GetController`))
  (bind _as_bp_ai_controller_master_0 (`self.As BP Ai Controller Master_0`))
  (`/Game/Blueprint/Character/CharacterMaster.NewPuceAttack` (stale `MeleeAttack` _ascharacter_master) self (`self.PressesNeeded`) :!label _label)
  (`/Engine/EditorBlueprintResources/StandardMacros.IsValid` _returnvalue
    (:`Is Valid`
      (`Controller.StopMovement` _returnvalue)
      (`self.K2_AttachToComponent` (`Character.Mesh` (stale `MeleeAttack` _ascharacter_master)) (`KismetArrayLibrary.Array_Random` (`self.SocketNames`)) "SnapToTarget" "KeepWorld" "KeepWorld" false)
      (`Controller.UnPossess` _returnvalue)
      (`AIPerceptionComponent.SetSenseEnabled` (`/Game/Blueprint/AI/AI_Puces/AIController/BP_AiControllerMaster.AIPerception` _as_bp_ai_controller_master_0) "/Script/AIModule.AISense_Sight" false)
      (`/Game/Blueprint/Character/CharacterMaster.NewAlertState` (stale `MeleeAttack` _ascharacter_master) _as_bp_ai_controller_master_0 2)
      (bind _outactors (`KismetSystemLibrary.SphereOverlapActors` (`self.K2_GetActorLocation`) 250.0 (`self.Object Types`) null (`|MakeArray` self :!type "Actor Object Reference")))
      (for _array_element _outactors
        (if (`KismetSystemLibrary.DoesImplementInterface` _array_element "/Game/Blueprint/BPI_Damageable.BPI_Damageable_C")
          (bind _ascharacter_master (cast `/Game/Blueprint/Character/CharacterMaster` _array_element))
          (bind _output_get (set `self.As Character Master_0` _ascharacter_master))
          (`/Game/Blueprint/Character/CharacterMaster.ReducePlayerSpeed` _output_get)
          (`self.ReportNoise`))))))

(event `MeleeAttack`
  (params (NewParam :type "Actor Object Reference"))
  (bind _ascharacter_master (cast `/Game/Blueprint/Character/CharacterMaster` NewParam))
  (if (not (!= _ascharacter_master (`GameplayStatics.GetPlayerCharacter` 0)))
    (goto _label)
    (else
      (switch `string` (`KismetSystemLibrary.GetDisplayName` _ascharacter_master)
        (:`BP_FirstChara`
          (`self.InCaseFirstCharaIsTargeted`))
        (:`BP_SecondChara`
          (`self.InCaseSecondCharaIsTargeted`))
        (:`BP_ThirdChara`
          (`self.InCaseThirdCharaIsTargeted`))))))

(event `self.Sphere.OnComponentBeginOverlap`
  (params (OverlappedComponent :type "PrimitiveComponent Object Reference") (OtherActor :type "Actor Object Reference") (OtherComp :type "PrimitiveComponent Object Reference") (OtherBodyIndex :type Integer) (bFromSweep :type Boolean) (SweepResult :type "HitResult Structure (by ref)"))
  (bind _ascharacter_master (cast `/Game/Blueprint/Character/CharacterMaster` OtherActor))
  (`self.MeleeAttack` _ascharacter_master))

(event `InCaseFirstCharaIsTargeted`
  ;[0 0 1] In case the player caught is not the same as the player controlled, we switch to the player that is being attacked
  (if (`KismetStringLibrary.EqualEqual_StrStr` (`KismetSystemLibrary.GetDisplayName` (`GameplayStatics.GetPlayerCharacter` 0)) "BP_SecondChara")
    (bind _asgame_mode_wardogs (`/Game/Blueprint/FL_Main.GetGameMode`))
    (set `/Game/Blueprint/GameMode/GameModeWardogs.IsSwitching` true _asgame_mode_wardogs)
    (`/Game/Blueprint/GameMode/GameModeWardogs.SwitchChara1` _asgame_mode_wardogs)
    (else
      (bind _asgame_mode_wardogs_2 (`/Game/Blueprint/FL_Main.GetGameMode`))
      (set `/Game/Blueprint/GameMode/GameModeWardogs.IsSwitching` true _asgame_mode_wardogs_2)
      (`/Game/Blueprint/GameMode/GameModeWardogs.SwitchChara0` _asgame_mode_wardogs_2)))
  (`self.ContinueMeleeAttack`))

(event `ReportNoise`
  (bind _as_character_master_0 (`self.As Character Master_0`))
  (if (not (`self.QTeIsComplete`))
    (`AISense_Hearing.ReportNoiseEvent` (`self.K2_GetActorLocation`) (`self.MeleeLoudness`) self)
    (`KismetSystemLibrary.Delay` 0.1)
    (`self.ReportNoise`)
    (else
      (bind _asmy_player_controller (`/Game/Blueprint/FL_Main.GetPlayerController`))
      (set `/Game/Blueprint/Character/MyPlayerController.IsBeingAttack` false _asmy_player_controller)
      (`/Game/Blueprint/Character/CharacterMaster.RestorePlayerSpeed` _as_character_master_0)
      (`/Game/Blueprint/Character/CharacterMaster.ResetAlertLevelUI` _as_character_master_0 (`self.As BP Ai Controller Master_0`))
      (`self.K2_DestroyActor`))))

(event `/Game/Blueprint/BPI_InteractWithEnnemy.InteractWithEnnemy`
  ;[0 1 0] desactiver pour les test
)

(event `InCaseSecondCharaIsTargeted`
  ;[0 0 1] In case the player caught is not the same as the player controlled, we switch to the player that is being attacked
  (if (`KismetStringLibrary.EqualEqual_StrStr` (`KismetSystemLibrary.GetDisplayName` (`GameplayStatics.GetPlayerCharacter` 0)) "BP_FirstChara")
    (bind _asgame_mode_wardogs (`/Game/Blueprint/FL_Main.GetGameMode`))
    (set `/Game/Blueprint/GameMode/GameModeWardogs.IsSwitching` true _asgame_mode_wardogs)
    (`/Game/Blueprint/GameMode/GameModeWardogs.SwitchChara0` _asgame_mode_wardogs)
    (else
      (bind _asgame_mode_wardogs_2 (`/Game/Blueprint/FL_Main.GetGameMode`))
      (set `/Game/Blueprint/GameMode/GameModeWardogs.IsSwitching` true _asgame_mode_wardogs_2)
      (`/Game/Blueprint/GameMode/GameModeWardogs.SwitchChara1` _asgame_mode_wardogs_2)))
  (`self.ContinueMeleeAttack`))

(event `/Game/Blueprint/BPI_InteractWithEnnemy.StopInteractWithEnnemy`
  ;[0 1 0] desactiver pour les test
)

(event `DecrementProgressBar`
  (bind _widgetref (`self.WidgetRef`))
  (bind _pressedamount (`self.PressedAmount`))
  ;[0 1 0] desactiver pour les test
  (bind _result (`/Engine/EditorBlueprintResources/StandardMacros.DecrementFloat` _pressedamount)
    (:`  `
      (bind _output_get (set `self.PressedAmount` (`KismetMathLibrary.FClamp` _result 0.0 _pressedamount)))
      (`/Engine/EditorBlueprintResources/StandardMacros.IsValid` _widgetref
        (:`Is Valid`
          (set `/Game/UI/SpamE/W_SpamE.AmountPressed` _output_get _widgetref)
          (if (<= (`self.PressedAmount`) 0.0)
            (`KismetSystemLibrary.K2_ClearAndInvalidateTimerHandle` (`self.TimerDecrementProgressBarRef`))))))))

(event `InCaseThirdCharaIsTargeted`
  ;[0 0 1] In case the player caught is not the same as the player controlled, we switch to the player that is being attacked
  (if (`KismetStringLibrary.EqualEqual_StrStr` (`KismetSystemLibrary.GetDisplayName` (`GameplayStatics.GetPlayerCharacter` 0)) "BP_FirstChara")
    (bind _asgame_mode_wardogs (`/Game/Blueprint/FL_Main.GetGameMode`))
    (set `/Game/Blueprint/GameMode/GameModeWardogs.IsSwitching` true _asgame_mode_wardogs)
    (`/Game/Blueprint/GameMode/GameModeWardogs.SwitchChara1` _asgame_mode_wardogs)
    (else
      (bind _asgame_mode_wardogs_2 (`/Game/Blueprint/FL_Main.GetGameMode`))
      (set `/Game/Blueprint/GameMode/GameModeWardogs.IsSwitching` true _asgame_mode_wardogs_2)
      (`/Game/Blueprint/GameMode/GameModeWardogs.SwitchChara0` _asgame_mode_wardogs_2)))
  (`self.ContinueMeleeAttack`))

(fn `UserConstructionScript`
  (`parent.UserConstructionScript`))