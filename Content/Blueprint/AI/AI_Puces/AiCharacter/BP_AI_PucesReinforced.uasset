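; Reinforced Puces AI enemy that latches on when a player character overlaps its sphere, starting a quick-time event as an explosive attack.
; It stops and unpossesses itself, slows damageable characters nearby, then loops a warning sound while a one-shot timer counts down to a damaging explosion.
; A successful HUD QTE result cancels the timer, restores speed and destroys it.
; An older press-counter progress bar remains unwired.
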(event `self.ReceiveBeginPlay`
  (`parent.ReceiveBeginPlay`)
  (add `/Game/UI/UI_InGame/UI_QTE/UI_QTE.FinishQTE` (`/Game/UI/UI_InGame/Widget_HeadUp.UI_QTE` (`self.W_HeadUpRef`)) (delegate `QTEFinish`)))

(event `QTEFinish`
  (params (`Succes?` :type Boolean) (Caller :type "Actor Object Reference"))
  (if (== Caller self)
    (set `self.QTeIsComplete` `Succes?`)))

(event `/Game/Blueprint/AI/AI_Puces/BPI_ChangeAiStates.ChangeState`
  (params (AlertState :type "/Game/Blueprint/AI/AI_Puces/E_AIStates Enum" :default "NewEnumerator1"))
  (`parent.ChangeState` AlertState))

(event `/Game/Blueprint/BPI_Damageable.TakeDamage`
  (params (Damage :type "Float (single-precision)"))
  (`parent.TakeDamage` Damage))

(event `ExplosiveAttack`
  (params (NewParam :type "Actor Object Reference"))
  (bind _returnvalue (`self.GetController`))
  (bind _ascharacter_master (cast `/Game/Blueprint/Character/CharacterMaster` NewParam))
  (`/Game/Blueprint/Character/CharacterMaster.NewPuceAttack` _ascharacter_master self (`self.PressesNeeded`))
  (`/Engine/EditorBlueprintResources/StandardMacros.IsValid` _returnvalue
    (:`Is Valid`
      (`Controller.StopMovement` _returnvalue)
      (`self.K2_AttachToComponent` null "None" "SnapToTarget" "KeepWorld" "KeepWorld")
      (`Controller.UnPossess` _returnvalue)
      (bind _outactors (`KismetSystemLibrary.SphereOverlapActors` (`self.K2_GetActorLocation`) 250.0 (`self.Object Types`) null (`|MakeArray` self :!type "Actor Object Reference")))
      (for _array_element _outactors
        (if (`KismetSystemLibrary.DoesImplementInterface` _array_element "/Game/Blueprint/BPI_Damageable.BPI_Damageable_C")
          (bind _ascharacter_master_2 (cast `/Game/Blueprint/Character/CharacterMaster` _array_element))
          (bind _output_get (set `self.As Character Master_0` _ascharacter_master_2))
          (`/Game/Blueprint/Character/CharacterMaster.ReducePlayerSpeed` _output_get)
          (if (not (`self.QTeIsComplete`))
            (`self.LaunchExplosion`)))))))

(event `self.Sphere.OnComponentBeginOverlap`
  (params (OverlappedComponent :type "PrimitiveComponent Object Reference") (OtherActor :type "Actor Object Reference") (OtherComp :type "PrimitiveComponent Object Reference") (OtherBodyIndex :type Integer) (bFromSweep :type Boolean) (SweepResult :type "HitResult Structure (by ref)"))
  (bind _ascharacter_master (cast `/Game/Blueprint/Character/CharacterMaster` OtherActor))
  (`self.ExplosiveAttack` _ascharacter_master))

(event `LaunchExplosion`
  (if (not (`self.QTeIsComplete`))
    (`GameplayStatics.PlaySoundAtLocation` null (`self.K2_GetActorLocation`) (struct) 1.0 1.0 0.0 null null null)
    (`KismetSystemLibrary.Delay` 0.2)
    (`self.LaunchExplosion`)
    (`/Engine/EditorBlueprintResources/StandardMacros.DoOnce` false
      (:`Completed`
        (bind _returnvalue (`KismetSystemLibrary.K2_SetTimerDelegate` (delegate `StartExplosion`) 5.0))
        (set `self.ExplosionTimerRef` _returnvalue)))
    (else
      (`KismetSystemLibrary.K2_ClearAndInvalidateTimerHandle` (`self.ExplosionTimerRef`))
      (`/Game/Blueprint/Character/CharacterMaster.RestorePlayerSpeed` (`self.As Character Master_0`))
      (bind _asmy_player_controller (`/Game/Blueprint/FL_Main.GetPlayerController`))
      (set `/Game/Blueprint/Character/MyPlayerController.IsBeingAttack` false _asmy_player_controller)
      (`self.K2_DestroyActor`))))

(event `StartExplosion`
  (`NiagaraFunctionLibrary.SpawnSystemAttached` null null "None" (`self.K2_GetActorLocation`) (struct) "KeepRelativeOffset")
  (`KismetSystemLibrary.PrintString` "ExplosiveAttack")
  (message `/Game/Blueprint/BPI_Damageable.TakeDamage` (stale `ExplosiveAttack` _array_element) 110.0))

(event `/Game/Blueprint/BPI_InteractWithEnnemy.InteractWithEnnemy`
  ;[1 1 1] desactiver
)

(event `/Game/Blueprint/BPI_InteractWithEnnemy.StopInteractWithEnnemy`
  ;[1 1 1] desactiver
)

(event `DecrementProgressBar`
  (bind _pressedamount (`self.PressedAmount`))
  ;[1 1 1] desactiver
  (bind _result (`/Engine/EditorBlueprintResources/StandardMacros.DecrementFloat` _pressedamount)
    (:`  `
      (bind _output_get (set `self.PressedAmount` (`KismetMathLibrary.FClamp` _result 0.0 _pressedamount)))
      (set `/Game/UI/SpamE/W_SpamE.AmountPressed` _output_get (`self.WidgetRef`))
      (if (<= (`self.PressedAmount`) 0.0)
        (`KismetSystemLibrary.K2_ClearAndInvalidateTimerHandle` (`self.TimerDecrementProgressBarRef`))))))

(fn `UserConstructionScript`
  (`parent.UserConstructionScript`))