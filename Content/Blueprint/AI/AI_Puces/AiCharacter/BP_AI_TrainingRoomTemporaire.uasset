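; Temporary training-room variant of the Puce AI enemy, with melee attack, overlap and player interaction overridden as empty.
; On BeginPlay it binds to BP_RelaySound, whose event toggles melee loudness between full and half.
; The latch-on attack, which attaches to the player, slows them and repeats noise reports until a button-mash QTE completes, remains as disconnected logic, so nothing here starts it.
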(event `self.ReceiveBeginPlay`
  (`parent.ReceiveBeginPlay`)
  (bind _returnvalue (`GameplayStatics.GetActorOfClass` "/Game/Blueprint/WorldMechanics/Relay/BP_RelaySound.BP_RelaySound_C"))
  (`/Engine/EditorBlueprintResources/StandardMacros.IsValid` _returnvalue
    (:`Is Valid`
      (add `/Game/Blueprint/WorldMechanics/Relay/BP_RelaySound.RiseAiMeleeAttackLoudness` _returnvalue (delegate `RiseMeleeLoudness`)))))

(event `RiseMeleeLoudness`
  (`/Engine/EditorBlueprintResources/StandardMacros.FlipFlop`
    (:`A`
      (set `self.MeleeLoudness` 1.0))
    (:`B`
      (set `self.MeleeLoudness` 0.5))))

(event `/Game/Blueprint/AI/AI_Puces/BPI_ChangeAiStates.ChangeState`
  (params (AlertState :type "/Game/Blueprint/AI/AI_Puces/E_AIStates Enum" :default "NewEnumerator1"))
  (`parent.ChangeState` AlertState))

(event `/Game/Blueprint/BPI_Damageable.TakeDamage`
  (params (Damage :type "Float (single-precision)"))
  (`parent.TakeDamage` Damage))

(event `MeleeAttack`
  (params (NewParam :type "Actor Object Reference")))

(event `self.Sphere.OnComponentBeginOverlap`
  (params (OverlappedComponent :type "PrimitiveComponent Object Reference") (OtherActor :type "Actor Object Reference") (OtherComp :type "PrimitiveComponent Object Reference") (OtherBodyIndex :type Integer) (bFromSweep :type Boolean) (SweepResult :type "HitResult Structure (by ref)")))

(event `ReportNoise`
  (if (not (`self.QTeIsComplete`))
    (`AISense_Hearing.ReportNoiseEvent` (`self.K2_GetActorLocation`) (`self.MeleeLoudness`) self)
    (`KismetSystemLibrary.Delay` 0.1)
    (`self.ReportNoise`)
    (else
      (bind _asmy_player_controller (`/Game/Blueprint/FL_Main.GetPlayerController`))
      (set `/Game/Blueprint/Character/MyPlayerController.IsBeingAttack` false _asmy_player_controller)
      (`/Game/Blueprint/Character/CharacterMaster.RestorePlayerSpeed` (`self.As Character Master_0`))
      (`self.K2_DestroyActor`))))

(event `/Game/Blueprint/BPI_InteractWithEnnemy.InteractWithEnnemy`
  ;[0 1 0] desactiver pour les test
)

(event `/Game/Blueprint/BPI_InteractWithEnnemy.StopInteractWithEnnemy`
  ;[0 1 0] desactiver pour les test
)

(event `DecrementProgressBar`
  (bind _widgetref (`self.WidgetRef`))
  (bind _pressedamount (`self.PressedAmount`))
  ;[0 1 0] desactiver pour les test
  (bind _result (`/Engine/EditorBlueprintResources/StandardMacros.DecrementFloat` _pressedamount)
    (:`  `
      (bind _output_get (set `self.PressedAmount` (`KismetMathLibrary.FClamp` _result 0.0 _pressedamount)))
      (`/Engine/EditorBlueprintResources/StandardMacros.IsValid` _widgetref
        (:`Is Valid`
          (set `/Game/UI/SpamE/W_SpamE.AmountPressed` _output_get _widgetref)
          (if (<= (`self.PressedAmount`) 0.0)
            (`KismetSystemLibrary.K2_ClearAndInvalidateTimerHandle` (`self.TimerDecrementProgressBarRef`))))))))

(fn `UserConstructionScript`
  (`parent.UserConstructionScript`))