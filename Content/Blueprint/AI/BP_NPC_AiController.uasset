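; AI controller for patrolling NPCs that runs the BT_NPC_AI behavior tree.
; On BeginPlay it seeds the blackboard with loop, direction and wait time settings, drawing on the controlled NPC's patrol path.
; Sight perception sets CanSeePlayer whenever a CharacterMaster is sensed or lost.
; Paralized and Stuned events halt movement and logic, then restart the tree after a delay; Paralized also clears CanSeePlayer.
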(event `self.ReceiveBeginPlay`
  (`self.RunBehaviorTree` "/Game/Blueprint/AI/BT_NPC_AI.BT_NPC_AI")
  (bind _asbp_npc_ai (cast `/Game/Blueprint/AI/BP_NPC_Ai` (`self.K2_GetPawn`)))
  (bind _output_get (set `self.NPC_AiRef` _asbp_npc_ai))
  (`BlackboardComponent.SetValueAsBool` (`AIBlueprintHelperLibrary.GetBlackboard` null) "PathLooping" (`/Game/Blueprint/AI/BP_PatrolPath.IsLooping` (`/Game/Blueprint/AI/BP_NPC_Ai.PatrolPath` _output_get)))
  (`BlackboardComponent.SetValueAsInt` (`AIBlueprintHelperLibrary.GetBlackboard` null) "Direction" 1)
  (`BlackboardComponent.SetValueAsFloat` (`AIBlueprintHelperLibrary.GetBlackboard` null) "WaitTime" (`/Game/Blueprint/AI/BP_PatrolPath.WaitTime` (`/Game/Blueprint/AI/BP_NPC_Ai.PatrolPath` (`self.NPC_AiRef`)))))

(event `self.AIPerception_Sight.OnTargetPerceptionUpdated`
  (params (Actor :type "Actor Object Reference") (Stimulus :type "AIStimulus Structure"))
  (cast `/Game/Blueprint/Character/CharacterMaster` Actor)
  (`BlackboardComponent.SetValueAsBool` (`AIBlueprintHelperLibrary.GetBlackboard` null) "CanSeePlayer" (`.bSuccessfullySensed` (break `AIStimulus` Stimulus))))

(event `Paralized`
  (params (Time :type "Float (double-precision)"))
  ;[0 1 0] Paralized System
  (`BlackboardComponent.SetValueAsBool` (`AIBlueprintHelperLibrary.GetBlackboard` null) "CanSeePlayer" false)
  (`self.StopMovement`)
  (`BrainComponent.StopLogic` (`self.BrainComponent`) "")
  (`KismetSystemLibrary.Delay` Time)
  (`self.RunBehaviorTree` "/Game/Blueprint/AI/BT_NPC_AI.BT_NPC_AI"))

(event `Stuned`
  (params (Time :type "Float (double-precision)"))
  ;[0 1 0] Stuned System
  (`self.StopMovement`)
  (`BrainComponent.StopLogic` (`self.BrainComponent`) "")
  (`KismetSystemLibrary.Delay` Time)
  (`self.RunBehaviorTree` "/Game/Blueprint/AI/BT_NPC_AI.BT_NPC_AI"))

(fn `UserConstructionScript`)