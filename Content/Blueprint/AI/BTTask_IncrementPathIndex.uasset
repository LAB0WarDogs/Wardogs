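; Behavior Tree task that advances an AI's patrol path index while the Blackboard direction is forward (1).
; It casts the controlled pawn to BP_AI_Master and checks the next index against the length of its PatrolPath points.
; Within bounds it stores the new index and succeeds; past the last point it flips direction to -1 and fails.
; Any other direction fails immediately, while a failed cast never finishes the task.
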(event `self.ReceiveExecuteAI`
  (params (OwnerController :type "AIController Object Reference") (ControlledPawn :type "Pawn Object Reference"))
  (bind _returnvalue (+ (`BTFunctionLibrary.GetBlackboardValueAsInt` (`self.BB_PathIndex`)) 1))
  (if (== (`BTFunctionLibrary.GetBlackboardValueAsInt` (`self.BB_Direction`)) 1)
    (bind _asbp_ai_master (cast `/Game/Blueprint/AI/AI_Puces/AiCharacter/BP_AI_Master` ControlledPawn))
    (if (<= _returnvalue (- (`KismetArrayLibrary.Array_Length` (`/Game/Blueprint/AI/BP_PatrolPath.PathPoint` (`/Game/Blueprint/AI/AI_Puces/AiCharacter/BP_AI_Master.PatrolPath` _asbp_ai_master))) 1))
      (`BTFunctionLibrary.SetBlackboardValueAsInt` (`self.BB_Direction`) 1)
      (`BTFunctionLibrary.SetBlackboardValueAsInt` (`self.BB_PathIndex`) _returnvalue)
      (`self.FinishExecute` true)
      (else
        (`BTFunctionLibrary.SetBlackboardValueAsInt` (`self.BB_Direction`) -1)
        (`self.FinishExecute` false)))
    (else
      (`self.FinishExecute` false))))