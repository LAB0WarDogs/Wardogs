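; Behavior tree task that writes an AI's next patrol point to the blackboard.
; On execute it casts the controlled pawn to BP_AI_Master and reads the point at the blackboard path index from its PatrolPath.
; That point is converted from the path actor's local space to world space and stored in the path vector key.
; The task finishes only when the cast succeeds and the path is valid, with no failure branch.
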(event `self.ReceiveExecuteAI`
  (params (OwnerController :type "AIController Object Reference") (ControlledPawn :type "Pawn Object Reference"))
  (bind _asbp_ai_master (cast `/Game/Blueprint/AI/AI_Puces/AiCharacter/BP_AI_Master` ControlledPawn))
  (bind _patrolpath (`/Game/Blueprint/AI/AI_Puces/AiCharacter/BP_AI_Master.PatrolPath` _asbp_ai_master)
    (:`then`
      (`BTFunctionLibrary.SetBlackboardValueAsVector` (`self.BB_PathVector`) (`KismetMathLibrary.TransformLocation` (`Actor.GetTransform` _patrolpath) (`|GetArrayItem` (`/Game/Blueprint/AI/BP_PatrolPath.PathPoint` _patrolpath) (`BTFunctionLibrary.GetBlackboardValueAsInt` (`self.BB_PathIndex`)))))
      (`self.FinishExecute` true))
    (:`else`)))