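; Skill component for the third character that lets the player preview and place a BP_Trap.
; Activation consumes a charge, flags the character as using a skill and shows its Piege preview, then confirming spawns the trap there.
; Cancel hides the preview and refunds the charge, but TrapHasBeenSet is never cleared here, blocking cancel after the first placement.
; CoolDown, not called within this graph, starts the CharacterMaster cooldown and restores the charge after a delay.
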(event `self.ReceiveBeginPlay`
  (bind _returnvalue (`GameplayStatics.GetActorOfClass` "/Game/Blueprint/Character/BP_ThirdChara.BP_ThirdChara_C"))
  (set `self.Third Chara Ref` _returnvalue)
  (bind _ascharacter_master (`/Game/Blueprint/FL_Main.Get Player Character Master`))
  (set `self.As Character Master` _ascharacter_master))

(event `ActivateThirdSkill`
  (bind _third_chara_ref (`self.Third Chara Ref`))
  (if (and (not (`/Game/Blueprint/Character/CharacterMaster.IsUsingSkill` (`self.Third Chara Ref`))) (> (`self.TrapCount`) 0))
    (set `/Game/Blueprint/Character/CharacterMaster.IsUsingSkill` true _third_chara_ref)
    (set `/Game/Blueprint/Character/CharacterMaster.CanMoveWithUsingSkill` true _third_chara_ref)
    (set `self.TrapCount` (- (`self.TrapCount`) 1))
    (`self.PreviewPos`)))

(event `PreviewPos`
  (`SceneComponent.SetVisibility` (`/Game/Blueprint/Character/BP_ThirdChara.Piege` (`self.Third Chara Ref`)) true false))

(event `UsingSecondSkill`
  (bind _third_chara_ref (`self.Third Chara Ref`))
  (bind _third_chara_ref_2 (`self.Third Chara Ref`))
  (if (`/Game/Blueprint/Character/CharacterMaster.IsUsingSkill` (`self.Third Chara Ref`))
    (set `self.TrapHasBeenSet` true)
    (`|SpawnActorFromClass` "/Game/Blueprint/Actors/Trap/BP_Trap.BP_Trap_C" (`KismetMathLibrary.MakeTransform` (`SceneComponent.K2_GetComponentLocation` (`/Game/Blueprint/Character/BP_ThirdChara.Piege` _third_chara_ref)) (`Actor.K2_GetActorRotation` _third_chara_ref)) "Undefined" "OverrideRootScale" null null)
    (set `/Game/Blueprint/Character/CharacterMaster.IsUsingSkill` false _third_chara_ref_2)
    (set `/Game/Blueprint/Character/CharacterMaster.CanMoveWithUsingSkill` false _third_chara_ref_2)
    (`SceneComponent.SetVisibility` (`/Game/Blueprint/Character/BP_ThirdChara.Piege` (`self.Third Chara Ref`)) false false)))

(event `CancelTrapSkill`
  (bind _third_chara_ref (`self.Third Chara Ref`))
  (if (not (`self.TrapHasBeenSet`))
    (set `/Game/Blueprint/Character/CharacterMaster.IsUsingSkill` false _third_chara_ref)
    (set `/Game/Blueprint/Character/CharacterMaster.CanMoveWithUsingSkill` false _third_chara_ref)
    (`SceneComponent.SetVisibility` (`/Game/Blueprint/Character/BP_ThirdChara.Piege` (`self.Third Chara Ref`)) false false)
    (set `self.TrapCount` 1 :!label _label)))

(event `CoolDown`
  (bind _cooldownbeforeactifagain (`self.CooldownBeforeActifAgain`))
  (`/Game/Blueprint/Character/CharacterMaster.StartCooldown` (`self.As Character Master`) _cooldownbeforeactifagain)
  (`KismetSystemLibrary.Delay` _cooldownbeforeactifagain)
  (goto _label))