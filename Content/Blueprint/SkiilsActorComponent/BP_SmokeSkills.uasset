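; Smoke skill component for BP_ThirdChara: aims and throws a BP_Smoke projectile, then starts a cooldown unless cancelled.
; Aiming slows time, locks the camera, turns the character toward a mouse/joystick-driven cursor target and colours it red or green by range.
; Launch speed equals the cursor hit's distance from the player, shared by throw and preview.
; Self-recalling delayed events refresh facing, range and a predicted arc of reused AimPoints actors.
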(event `self.ReceiveBeginPlay`
  (bind _returnvalue (`GameplayStatics.GetActorOfClass` "/Game/Blueprint/Character/BP_ThirdChara.BP_ThirdChara_C"))
  (set `self.Third Chara Ref` _returnvalue)
  (set `self.Smoke Target` (`/Game/Blueprint/Character/BP_ThirdChara.SmokeTarget` _returnvalue))
  (set `self.Smoke Ref` (`/Game/Blueprint/Character/BP_ThirdChara.SmokeRef` _returnvalue)))

(event `self.ReceiveTick`
  (params (DeltaSeconds :type "Float (single-precision)"))
  (bind (_sizex _sizey) (`PlayerController.GetViewportSize` (`GameplayStatics.GetPlayerController` 0)))
  (bind _asmy_player_controller (`/Game/Blueprint/FL_Main.GetPlayerController`))
  (bind (_locationx _locationy) (`PlayerController.GetMousePosition` _asmy_player_controller))
  (`PlayerController.SetMouseLocation` (`GameplayStatics.GetPlayerController` 0) (`KismetMathLibrary.Clamp` (`KismetMathLibrary.FTrunc` (+ _locationx (* (`/Game/Blueprint/Character/MyPlayerController.JoystickX` _asmy_player_controller) 20.0))) 0 _sizex) (`KismetMathLibrary.Clamp` (`KismetMathLibrary.FTrunc` (+ _locationy (* (`/Game/Blueprint/Character/MyPlayerController.JoystickY` _asmy_player_controller) 20.0))) 0 _sizey))
  (`KismetSystemLibrary.MoveComponentTo` (`self.Smoke Target`) (`.ImpactPoint` (`GameplayStatics.BreakHitResult` (`PlayerController.GetHitResultUnderCursorByChannel` (`GameplayStatics.GetPlayerController` 0) "TraceTypeQuery1" true))) (struct :`Pitch` -90.0) false false 0.1))

(event `ActivateFirstSkill`
  (bind _third_chara_ref (`self.Third Chara Ref`))
  (if (and (not (`/Game/Blueprint/Character/CharacterMaster.IsUsingSkill` (`self.Third Chara Ref`))) (`self.CoolDownIsOver`))
    (set `/Game/Blueprint/Character/CharacterMaster.IsUsingSkill` true (`self.Third Chara Ref`))
    (set `/Game/Blueprint/Character/CharacterMaster.CanMoveWithUsingSkill` true _third_chara_ref)
    (set `/Game/Blueprint/Character/CharacterMaster.CantMoveCamera` true _third_chara_ref)
    (`self.SetComponentTickEnabled` true)
    (`self.AimingFirstSkill`)))

(event `AimingFirstSkill`
  (bind _smoke_target (`self.Smoke Target`))
  (bind (_sizex _sizey) (`PlayerController.GetViewportSize` (`GameplayStatics.GetPlayerController` 0)))
  (`|ExecutionSequence`
    (:`then_0`
      (set `self.FacePlayer?` true)
      (`self.FacePlayer`)
      (`SceneComponent.SetVisibility` _smoke_target true true)
      (`SceneComponent.K2_DetachFromComponent` _smoke_target "KeepWorld" "KeepWorld" "KeepWorld" true)
      (`PlayerController.SetMouseLocation` (`GameplayStatics.GetPlayerController` 0) (/ _sizex 2) (/ _sizey 2))
      (`GameplayStatics.SetGlobalTimeDilation` 0.5))
    (:`then_1`
      (set `self.IsAiming?` true)
      (`self.predict`))
    (:`then_2`
      (`self.get position`))))

(event `Cancelation`
  (bind _aimpoints (`self.AimPoints`))
  (bind _cooldownduration (`self.CoolDownDuration`))
  (bind _third_chara_ref (`self.Third Chara Ref`))
  (set `self.IsCanceled` true)
  (set `/Game/Blueprint/Character/CharacterMaster.IsUsingSkill` false (`self.Third Chara Ref`) :!label _label)
  (set `/Game/Blueprint/Character/CharacterMaster.CanMoveWithUsingSkill` false _third_chara_ref)
  (set `/Game/Blueprint/Character/CharacterMaster.CantMoveCamera` false _third_chara_ref)
  (set `self.IsAiming?` false)
  (`|ExecutionSequence`
    (:`then_0`
      (set `self.FacePlayer?` false)
      (`SceneComponent.SetVisibility` (`self.Smoke Target`) false true)
      (`GameplayStatics.SetGlobalTimeDilation` 1.0)
      (if (not (`self.IsCanceled`))
        (`/Game/Blueprint/Character/CharacterMaster.StartCooldown` (`self.Third Chara Ref`) _cooldownduration)
        (`KismetSystemLibrary.Delay` _cooldownduration))
      (`self.SetComponentTickEnabled` false)
      (set `self.CoolDownIsOver` true)
      (set `self.IsCanceled` false))
    (:`then_1`
      ;[1 1 1] Aim Visibility
      (for _array_element _aimpoints
        (`Actor.K2_DestroyActor` _array_element))
      (`KismetArrayLibrary.Array_Clear` _aimpoints))))

(event `UsingFirstSkill`
  (if (and (`/Game/Blueprint/Character/CharacterMaster.IsUsingSkill` (`self.Third Chara Ref`)) (`self.IsInRange`))
    (set `self.CoolDownIsOver` false)
    (bind _returnvalue (`|SpawnActorFromClass` "/Game/Blueprint/Actors/Smoke/BP_Smoke.BP_Smoke_C" (`KismetMathLibrary.MakeTransform` (`SceneComponent.K2_GetComponentLocation` (`self.Smoke Ref`)) (`Actor.K2_GetActorRotation` (`self.Third Chara Ref`))) "Undefined" "OverrideRootScale" null null))
    (`PrimitiveComponent.SetPhysicsLinearVelocity` (`/Game/Blueprint/Actors/Smoke/BP_Smoke.Sphere` _returnvalue) (* (`KismetMathLibrary.GetDirectionUnitVector` (`Actor.K2_GetActorLocation` (`self.Third Chara Ref`)) (`Actor.K2_GetActorLocation` _returnvalue)) (`self.GetSpeedBaseDistanceFromPlayer`)) true "None")
    (goto _label)))

(event `FacePlayer`
  (bind (_returnvalue_roll _returnvalue_pitch _returnvalue_yaw) (`KismetMathLibrary.BreakRotator` (`KismetMathLibrary.RInterpTo` (`Actor.K2_GetActorRotation` (`self.Third Chara Ref`)) (`KismetMathLibrary.FindLookAtRotation` (`Actor.K2_GetActorLocation` (`self.Third Chara Ref`)) (`.ImpactPoint` (`GameplayStatics.BreakHitResult` (`PlayerController.GetHitResultUnderCursorByChannel` (`GameplayStatics.GetPlayerController` 0) "TraceTypeQuery1" true)))) (`GameplayStatics.GetWorldDeltaSeconds`) 20.0)))
  (if (`self.FacePlayer?`)
    (`Actor.K2_SetActorRelativeRotation` (`self.Third Chara Ref`) (`KismetMathLibrary.MakeRotator` 0.0 0.0 _returnvalue_yaw) false false)
    (`KismetSystemLibrary.Delay` 0.001)
    (`self.FacePlayer`)))

(event `get position`
  (bind (_returnvalue_x _returnvalue_y) (`KismetMathLibrary.BreakVector` (`SceneComponent.K2_GetComponentLocation` (`self.Smoke Target`))))
  (bind (_returnvalue_x_2 _returnvalue_y_2) (`KismetMathLibrary.BreakVector` (`SceneComponent.K2_GetComponentLocation` (`Actor.RootComponent` (`self.Third Chara Ref`)))))
  (if (and (> (`KismetMathLibrary.Sqrt` (+ (`KismetMathLibrary.Square` (- _returnvalue_x _returnvalue_x_2)) (`KismetMathLibrary.Square` (- _returnvalue_y _returnvalue_y_2)))) (`self.Speed`)) (`self.IsAiming?`))
    (`PrimitiveComponent.SetMaterial` (`self.Smoke Target`) 0 "/Engine/EngineDebugMaterials/VertexColorViewMode_RedOnly.VertexColorViewMode_RedOnly")
    (set `self.IsInRange` false)
    (else
      (`PrimitiveComponent.SetMaterial` (`self.Smoke Target`) 0 "/Engine/EngineDebugMaterials/VertexColorViewMode_GreenOnly.VertexColorViewMode_GreenOnly")
      (set `self.IsInRange` true)))
  (`KismetSystemLibrary.Delay` 0.2)
  (`self.get position`))

(event `predict`
  (bind _aimpoints (`self.AimPoints`))
  (bind _returnvalue (`SceneComponent.K2_GetComponentLocation` (`self.Smoke Ref`)))
  ;[1 1 1] Prediction
  (if (`self.IsAiming?`)
    (bind (_outhit _outpathpositions) (`GameplayStatics.Blueprint_PredictProjectilePath_ByObjectType` :`StartPos` _returnvalue :`LaunchVelocity` (* (`KismetMathLibrary.GetDirectionUnitVector` (`Actor.K2_GetActorLocation` (`self.Third Chara Ref`)) _returnvalue) (`self.GetSpeedBaseDistanceFromPlayer`)) :`ProjectileRadius` 20.0 :`ObjectTypes` (`|MakeArray` "ObjectTypeQuery1" :!type "EObjectTypeQuery Enum") :`SimFrequency` 10.0))
    (`|ExecutionSequence`
      (:`then_0`
        (for (_array_element _array_index) _outpathpositions
          (if (> (`KismetMathLibrary.Conv_IntToDouble` _array_index) (`KismetMathLibrary.Conv_IntToDouble` (`KismetArrayLibrary.Array_LastIndex` _aimpoints)))
            (bind _returnvalue_2 (`|SpawnActorFromClass` "/Game/Blueprint/SkiilsActorComponent/AimPoints.AimPoints_C" (`KismetMathLibrary.MakeTransform` _array_element (struct) (0.1 0.1 0.1)) "Undefined" "OverrideRootScale" null null))
            (`KismetArrayLibrary.Array_Set` _aimpoints _array_index _returnvalue_2 true))))
      (:`then_1`
        (for (_array_element_2 _array_index_2) _aimpoints
          (if (>= (`KismetArrayLibrary.Array_LastIndex` _outpathpositions) _array_index_2)
            (bind _rootcomponent (`Actor.RootComponent` _array_element_2))
            (`SceneComponent.K2_SetWorldLocation` _rootcomponent (`|GetArrayItem` _outpathpositions _array_index_2) false true)
            (else
              (`SceneComponent.K2_SetWorldLocation` _rootcomponent (10000.0 0.0 0.0) false true)))))
      (:`then_2`
        (`KismetSystemLibrary.Delay` 0.01)
        (`self.predict`)))))

(fn `AlwaysFacePlayer`)

(fn `GetSpeedBaseDistanceFromPlayer`
  (returns (Speed :type "Float (double-precision)"))
  (return (`KismetMathLibrary.Vector_Distance` (`.ImpactPoint` (`GameplayStatics.BreakHitResult` (`PlayerController.GetHitResultUnderCursorByChannel` (`GameplayStatics.GetPlayerController` 0) "TraceTypeQuery1" true))) (`Actor.K2_GetActorLocation` (`self.Third Chara Ref`)))))