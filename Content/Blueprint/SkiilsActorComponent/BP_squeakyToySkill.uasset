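; Skill component for the second character that spawns a squeaky toy actor at that character's transform.
; On BeginPlay it caches the BP_SecondChara actor and the player's character master.
; Activation is gated by the character's IsUsingSkill flag and a local cooldown flag.
; Each use spawns the toy, clears the in-use flag, starts the cooldown on the character master and re-enables itself after a matching Delay.
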(event `self.ReceiveBeginPlay`
  (bind _returnvalue (`GameplayStatics.GetActorOfClass` "/Game/Blueprint/Character/BP_SecondChara.BP_SecondChara_C"))
  (set `self.SecondCharaRef` _returnvalue)
  (bind _ascharacter_master (`/Game/Blueprint/FL_Main.Get Player Character Master`))
  (set `self.As Character Master` _ascharacter_master))

(event `ActivateSecondSkill`
  (if (and (not (`/Game/Blueprint/Character/CharacterMaster.IsUsingSkill` (`self.SecondCharaRef`))) (`self.CooldownOver?`))
    (set `/Game/Blueprint/Character/CharacterMaster.IsUsingSkill` true (`self.SecondCharaRef`))
    (`self.UseSecondSkill`)))

(event `UseSecondSkill`
  (bind _cooldownbeforeactifagain (`self.CooldownBeforeActifAgain`))
  (if (`self.CooldownOver?`)
    (`|SpawnActorFromClass` "/Game/Blueprint/Actors/squeakyToy/BP_SkeaquyToy.BP_SkeaquyToy_C" (`Actor.GetTransform` (`self.SecondCharaRef`)) "Undefined" "OverrideRootScale" null null)
    (set `self.CooldownOver?` false)
    (set `/Game/Blueprint/Character/CharacterMaster.IsUsingSkill` false (`self.SecondCharaRef`))
    (`/Game/Blueprint/Character/CharacterMaster.StartCooldown` (`self.As Character Master`) _cooldownbeforeactifagain)
    (`KismetSystemLibrary.Delay` _cooldownbeforeactifagain)
    (set `self.CooldownOver?` true)))