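; Skill component for the third character (BP_ThirdChara) that remotely hacks a HackZone through a slow-motion aiming mode.
; Activation zooms, slows time and enables Tick, which moves the cursor with joystick input and eases a detached target component to the traced point.
; A second trace finds the hovered HackZone, triggers its glow and swaps two widgets.
; Use spends a battery, hacks, restores view and time, and clears skill flags only after cooldown.
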(event `self.ReceiveTick`
  (params (DeltaSeconds :type "Float (single-precision)"))
  (bind _as_bp_third_chara (`self.As BP Third Chara`))
  (bind _as_bp_third_chara_2 (`self.As BP Third Chara`))
  (bind (_sizex _sizey) (`PlayerController.GetViewportSize` (`GameplayStatics.GetPlayerController` 0)))
  (bind _asmy_player_controller (`/Game/Blueprint/FL_Main.GetPlayerController`))
  (bind (_locationx _locationy) (`PlayerController.GetMousePosition` _asmy_player_controller))
  (`PlayerController.SetMouseLocation` (`GameplayStatics.GetPlayerController` 0) (`KismetMathLibrary.Clamp` (`KismetMathLibrary.FTrunc` (+ _locationx (* (`/Game/Blueprint/Character/MyPlayerController.JoystickX` _asmy_player_controller) 20.0))) 0 _sizex) (`KismetMathLibrary.Clamp` (`KismetMathLibrary.FTrunc` (+ _locationy (* (`/Game/Blueprint/Character/MyPlayerController.JoystickY` _asmy_player_controller) 20.0))) 0 _sizey))
  (`KismetSystemLibrary.MoveComponentTo` (`self.Hack Comp Target`) (`.ImpactPoint` (`GameplayStatics.BreakHitResult` (`PlayerController.GetHitResultUnderCursorByChannel` (`GameplayStatics.GetPlayerController` 0) "TraceTypeQuery1" true))) (struct :`Pitch` -90.0) false false (* (`self.Over Time Speed`) (`GameplayStatics.GetWorldDeltaSeconds`)))
  (bind _ashack_zone (cast `/Game/Blueprint/WorldMechanics/Hack/HackZone` (`.HitActor` (`GameplayStatics.BreakHitResult` (`PlayerController.GetHitResultUnderCursorByChannel` (`GameplayStatics.GetPlayerController` 0) "TraceTypeQuery4" true))))
    (:`then`
      (bind _output_get (set `self.As Hack Zone` _ashack_zone))
      (`/Game/Blueprint/WorldMechanics/Hack/HackZone.GlowEffect` _output_get)
      (`SceneComponent.SetVisibility` (`/Game/Blueprint/Character/BP_ThirdChara.Widget_0` _as_bp_third_chara_2) false false)
      (`SceneComponent.SetVisibility` (`/Game/Blueprint/Character/BP_ThirdChara.Widget_1` _as_bp_third_chara_2) true false))
    (:`CastFailed`
      (set `self.As Hack Zone` null)
      (`SceneComponent.SetVisibility` (`/Game/Blueprint/Character/BP_ThirdChara.Widget_0` _as_bp_third_chara) true false)
      (`SceneComponent.SetVisibility` (`/Game/Blueprint/Character/BP_ThirdChara.Widget_1` _as_bp_third_chara) false false))))

(event `self.ReceiveBeginPlay`
  (`|ExecutionSequence`
    (:`then_0`
      (bind _returnvalue (`GameplayStatics.GetActorOfClass` "/Game/Blueprint/Character/BP_ThirdChara.BP_ThirdChara_C"))
      (bind _output_get (set `self.As BP Third Chara` _returnvalue))
      (set `self.Hack Comp Target` (`/Game/Blueprint/Character/BP_ThirdChara.HackCompTarget` _output_get)))
    (:`then_1`
      (bind _ascharacter_master (`/Game/Blueprint/FL_Main.Get Player Character Master`))
      (set `self.As Character Master` _ascharacter_master))))

(event `ActivateThirdSkill`
  (bind _as_bp_third_chara (`self.As BP Third Chara`))
  (if (and (not (`/Game/Blueprint/Character/CharacterMaster.IsUsingSkill` (`self.As BP Third Chara`))) (`self.CooldownIsOver`))
    (set `/Game/Blueprint/Character/CharacterMaster.IsUsingSkill` true _as_bp_third_chara)
    (set `/Game/Blueprint/Character/CharacterMaster.CanMoveWithUsingSkill` true _as_bp_third_chara)
    (`self.AimHackSkill`)))

(event `AimHackSkill`
  (bind _hack_comp_target (`self.Hack Comp Target`))
  (bind (_sizex _sizey) (`PlayerController.GetViewportSize` (`GameplayStatics.GetPlayerController` 0)))
  (`SceneComponent.SetVisibility` _hack_comp_target true true)
  (`SceneComponent.K2_DetachFromComponent` _hack_comp_target "KeepWorld" "KeepWorld" "KeepWorld" true)
  (`PlayerController.SetMouseLocation` (`GameplayStatics.GetPlayerController` 0) (/ _sizex 2) (/ _sizey 2))
  (`/Game/Blueprint/Character/BP_ThirdChara.Zoom` (`self.As BP Third Chara`))
  (`GameplayStatics.SetGlobalTimeDilation` 0.5)
  (`self.SetComponentTickEnabled` true))

(event `Cancelation`
  (bind _as_bp_third_chara (`self.As BP Third Chara`))
  (`GameplayStatics.SetGlobalTimeDilation` 1.0)
  (`self.SetComponentTickEnabled` false)
  (`SceneComponent.SetVisibility` (`self.Hack Comp Target`) false true)
  (set `/Game/Blueprint/Character/CharacterMaster.IsUsingSkill` false _as_bp_third_chara :!label _label)
  (set `/Game/Blueprint/Character/CharacterMaster.CanMoveWithUsingSkill` false _as_bp_third_chara))

(event `UseHackDistanceSkill`
  (bind _as_character_master (`self.As Character Master`))
  (bind _cooldown (`self.Cooldown`))
  (if (and (`/Game/Blueprint/Character/CharacterMaster.IsUsingSkill` (`self.As BP Third Chara`)) (`KismetSystemLibrary.IsValid` (`self.As Hack Zone`)))
    (`/Game/Blueprint/Character/CharacterMaster.UseBatteryFromInventory` _as_character_master)
    (set `self.CooldownIsOver` false)
    (`/Game/Blueprint/WorldMechanics/Hack/HackZone.HackDistance` (`self.As Hack Zone`))
    (`GameplayStatics.SetGlobalTimeDilation` 1.0)
    (`/Game/Blueprint/Character/BP_ThirdChara.Dezoom` (`self.As BP Third Chara`))
    (`SceneComponent.SetVisibility` (`self.Hack Comp Target`) false true)
    (`self.SetComponentTickEnabled` false)
    (`/Game/Blueprint/Character/CharacterMaster.StartCooldown` _as_character_master _cooldown)
    (`KismetSystemLibrary.Delay` _cooldown)
    (set `self.CooldownIsOver` true)
    (goto _label)))