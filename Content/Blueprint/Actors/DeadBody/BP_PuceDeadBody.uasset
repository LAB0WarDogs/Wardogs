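; BP_PuceDeadBody is a dead-body marker that sends AI to search for the killer when discovered.
; Initialization stores its owner and a search position, which switches to the marker's own location after a delay.
; After a brief delay, a box overlap by a non-owner BP_AI_Master triggers a one-time check that disables a sphere collision response and destroys the marker.
; That AI's controller then receives SearchPuceKiller with the stored position.
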(event `InitializationDeadBody`
  (params (Vector3 :type "Vector Structure") (Actor :type "Actor Object Reference"))
  (set `self.PuceOwner` Actor)
  (set `self.ChercheZone` Vector3)
  (`KismetSystemLibrary.Delay` (`self.DelayChercheZone`))
  (set `self.ChercheZone` (`self.K2_GetActorLocation` self)))

(event `CheckDeadBody`
  (set `self.Check` true)
  (`PrimitiveComponent.SetCollisionResponseToChannel` (`self.Sphere`) "ECC_GameTraceChannel4" "ECR_Ignore")
  (`self.K2_DestroyActor`))

(event `self.Box.OnComponentBeginOverlap`
  (params (OverlappedComponent :type "PrimitiveComponent Object Reference") (OtherActor :type "Actor Object Reference") (OtherComp :type "PrimitiveComponent Object Reference") (OtherBodyIndex :type Integer) (bFromSweep :type Boolean) (SweepResult :type "HitResult Structure (by ref)"))
  (`KismetSystemLibrary.Delay` 0.1)
  (if (!= OtherActor (`self.PuceOwner`))
    (bind _asbp_ai_master (cast `/Game/Blueprint/AI/AI_Puces/AiCharacter/BP_AI_Master` OtherActor))
    (bind _asbp_ai_controller_master (cast `/Game/Blueprint/AI/AI_Puces/AIController/BP_AiControllerMaster` (`AIBlueprintHelperLibrary.GetAIController` _asbp_ai_master)))
    (if (not (`self.Check`))
      (`self.CheckDeadBody`)
      (`/Game/Blueprint/AI/AI_Puces/AIController/BP_AiControllerMaster.SearchPuceKiller` _asbp_ai_controller_master (`self.ChercheZone`)))))

(fn `UserConstructionScript`)