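; Door actor that swings open and closed on interaction, with a widget shown while a CharacterMaster is in range.
; Interact requires CanOpen, while ForceOpen skips that check; both set the timeline rate from the open or close time based on IsOpen.
; A FlipFlop alternates playing and reversing the timeline, which yaws the Cylinder through 90 degrees and toggles IsOpen when finished.
; Box overlaps show the widget if IsWidgetNeeded and hide it on exit.
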(event `Force Open`
  ;[0 0 1] Comment
  (if (not (`self.IsOpen`)) :!label _label
    (`TimelineComponent.SetPlayRate` (`self.DoorTimeline`) (/ 1.0 (`self.TimeToOpen`)))
    (else
      (`TimelineComponent.SetPlayRate` (`self.DoorTimeline`) (/ 1.0 (`self.TimeToClose`)))))
  (`self.OpenDoor`))

(event `self.Interact`
  ;[0 0 1] Comment
  (if (`self.CanOpen`)
    (goto _label)))

(event `OpenDoor`
  ;[0 0 1] Comment
  (`/Engine/EditorBlueprintResources/StandardMacros.FlipFlop`
    (:`A`
      (bind (_direction _doortrack) (`Timeline|DoorTimeline` :!label _label_2)
        (:`Update`
          (`SceneComponent.K2_SetRelativeRotation` (`self.Cylinder`) (`KismetMathLibrary.MakeRotator` 0.0 0.0 (`KismetMathLibrary.Lerp` 0.0 -90.0 _doortrack)) false false))
        (:`Finished`
          (set `self.IsOpen` (not (`self.IsOpen`))))))
    (:`B`
      (goto _label_2 :!via `Reverse`))))

(event `self.Box.OnComponentBeginOverlap`
  (params (OverlappedComponent :type "PrimitiveComponent Object Reference") (OtherActor :type "Actor Object Reference") (OtherComp :type "PrimitiveComponent Object Reference") (OtherBodyIndex :type Integer) (bFromSweep :type Boolean) (SweepResult :type "HitResult Structure (by ref)"))
  ;[0 1 0] WidgetSystem
  (cast `/Game/Blueprint/Character/CharacterMaster` OtherActor)
  (if (`self.IsWidgetNeeded`)
    (`SceneComponent.SetVisibility` (`self.Widget`) true false)))

(event `self.Box.OnComponentEndOverlap`
  (params (OverlappedComponent :type "PrimitiveComponent Object Reference") (OtherActor :type "Actor Object Reference") (OtherComp :type "PrimitiveComponent Object Reference") (OtherBodyIndex :type Integer))
  ;[0 1 0] WidgetSystem
  (cast `/Game/Blueprint/Character/CharacterMaster` OtherActor)
  (`SceneComponent.SetVisibility` (`self.Widget`) false false))

(fn `UserConstructionScript`)