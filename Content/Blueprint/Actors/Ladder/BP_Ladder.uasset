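; BP_Ladder is an interactable ladder actor that toggles ladder state on the player character.
; Its Interact event sets NearLadder on the player's CharacterMaster, while the climbing itself is not handled here.
; A Box overlap shows the Widget component for any actor.
; When a CharacterMaster leaves the box, the ladder clears the player's NearLadder and OnLadder flags, restores Walking movement and hides the widget.
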(event `/Game/Blueprint/BPI_InteractInterface.Interact`
  (bind _ascharacter_master (`/Game/Blueprint/FL_Main.Get Player Character Master`))
  (set `/Game/Blueprint/Character/CharacterMaster.NearLadder` true _ascharacter_master))

(event `self.Box.OnComponentEndOverlap`
  (params (OverlappedComponent :type "PrimitiveComponent Object Reference") (OtherActor :type "Actor Object Reference") (OtherComp :type "PrimitiveComponent Object Reference") (OtherBodyIndex :type Integer))
  (cast `/Game/Blueprint/Character/CharacterMaster` OtherActor)
  (`|ExecutionSequence`
    (:`then_0`
      (bind _ascharacter_master (`/Game/Blueprint/FL_Main.Get Player Character Master`))
      (set `/Game/Blueprint/Character/CharacterMaster.NearLadder` false _ascharacter_master)
      (set `/Game/Blueprint/Character/CharacterMaster.OnLadder?` false _ascharacter_master)
      (`CharacterMovementComponent.SetMovementMode` (`Character.CharacterMovement` _ascharacter_master) "MOVE_Walking" 0))
    (:`then_1`
      ;[0 1 0] WidgetSystem
      (`SceneComponent.SetVisibility` (`self.Widget`) false false))))

(event `self.Box.OnComponentBeginOverlap`
  (params (OverlappedComponent :type "PrimitiveComponent Object Reference") (OtherActor :type "Actor Object Reference") (OtherComp :type "PrimitiveComponent Object Reference") (OtherBodyIndex :type Integer) (bFromSweep :type Boolean) (SweepResult :type "HitResult Structure (by ref)"))
  ;[0 1 0] WidgetSystem
  (`SceneComponent.SetVisibility` (`self.Widget`) true false))

(fn `UserConstructionScript`)