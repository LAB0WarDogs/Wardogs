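; BP_LadderV2 is a ladder actor that moves the player character along a spline when interacted with.
; Two trigger boxes, BoxAllez and BoxRetour, record whether the player is at the bottom or top and toggle a widget's visibility.
; Interact uses that position to call FollowSpline or ReverseSpline on the player character.
; Entering either box disables the opposite box's collision for a short delay.
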(event `/Game/Blueprint/BPI_InteractInterface.Interact`
  (switch `/Game/Blueprint/E_PlayerPosOnLadder` (`self.E_PosOnLadder`)
    (:`NewEnumerator0`
      (bind _ascharacter_master (`/Game/Blueprint/FL_Main.Get Player Character Master`))
      (`/Game/Blueprint/Character/CharacterMaster.FollowSpline` _ascharacter_master (`self.Spline`)))
    (:`NewEnumerator1`
      (bind _ascharacter_master_2 (`/Game/Blueprint/FL_Main.Get Player Character Master`))
      (`/Game/Blueprint/Character/CharacterMaster.ReverseSpline` _ascharacter_master_2 (`self.Spline`)))))

(event `self.BoxRetour.OnComponentBeginOverlap`
  (params (OverlappedComponent :type "PrimitiveComponent Object Reference") (OtherActor :type "Actor Object Reference") (OtherComp :type "PrimitiveComponent Object Reference") (OtherBodyIndex :type Integer) (bFromSweep :type Boolean) (SweepResult :type "HitResult Structure (by ref)"))
  (cast `/Game/Blueprint/Character/CharacterMaster` OtherActor)
  (set `self.E_PosOnLadder` "NewEnumerator1")
  (`SceneComponent.SetVisibility` (`self.Widget`) true false)
  (`PrimitiveComponent.SetCollisionEnabled` (`self.BoxAllez`) "NoCollision")
  (`KismetSystemLibrary.Delay` 5.0)
  (`PrimitiveComponent.SetCollisionEnabled` (`self.BoxAllez`) "QueryOnly"))

(event `self.BoxAllez.OnComponentBeginOverlap`
  (params (OverlappedComponent :type "PrimitiveComponent Object Reference") (OtherActor :type "Actor Object Reference") (OtherComp :type "PrimitiveComponent Object Reference") (OtherBodyIndex :type Integer) (bFromSweep :type Boolean) (SweepResult :type "HitResult Structure (by ref)"))
  (cast `/Game/Blueprint/Character/CharacterMaster` OtherActor)
  (set `self.E_PosOnLadder` "NewEnumerator0")
  (`SceneComponent.SetVisibility` (`self.Widget`) true false)
  (`PrimitiveComponent.SetCollisionEnabled` (`self.BoxRetour`) "NoCollision")
  (`KismetSystemLibrary.Delay` 5.0)
  (`PrimitiveComponent.SetCollisionEnabled` (`self.BoxRetour`) "QueryOnly"))

(event `self.BoxAllez.OnComponentEndOverlap`
  (params (OverlappedComponent :type "PrimitiveComponent Object Reference") (OtherActor :type "Actor Object Reference") (OtherComp :type "PrimitiveComponent Object Reference") (OtherBodyIndex :type Integer))
  (cast `/Game/Blueprint/Character/CharacterMaster` OtherActor)
  (`SceneComponent.SetVisibility` (`self.Widget`) false false :!label _label))

(event `self.BoxRetour.OnComponentEndOverlap`
  (params (OverlappedComponent :type "PrimitiveComponent Object Reference") (OtherActor :type "Actor Object Reference") (OtherComp :type "PrimitiveComponent Object Reference") (OtherBodyIndex :type Integer))
  (cast `/Game/Blueprint/Character/CharacterMaster` OtherActor)
  (goto _label))

(fn `UserConstructionScript`)