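; BP_SpamETest is a test interactable that is destroyed once the player's press count reaches a required amount.
; A CharacterMaster entering its box creates a W_SpamE widget showing the required presses, and leaving removes it.
; Interact increments the count and updates the widget, while StopInteracting waits through a retriggerable delay, then starts a looping timer that drains the count toward zero.
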(event `self.Box.OnComponentBeginOverlap`
  (params (OverlappedComponent :type "PrimitiveComponent Object Reference") (OtherActor :type "Actor Object Reference") (OtherComp :type "PrimitiveComponent Object Reference") (OtherBodyIndex :type Integer) (bFromSweep :type Boolean) (SweepResult :type "HitResult Structure (by ref)"))
  (cast `/Game/Blueprint/Character/CharacterMaster` OtherActor)
  (bind _returnvalue (`|CreateWidget` "/Game/UI/SpamE/W_SpamE.W_SpamE_C"))
  (bind _output_get (set `self.WidgetRef` _returnvalue))
  (`UserWidget.AddToViewport` _output_get 0)
  (set `/Game/UI/SpamE/W_SpamE.PressesNeeded` (`self.PressesNeeded`) _output_get))

(event `self.Box.OnComponentEndOverlap`
  (params (OverlappedComponent :type "PrimitiveComponent Object Reference") (OtherActor :type "Actor Object Reference") (OtherComp :type "PrimitiveComponent Object Reference") (OtherBodyIndex :type Integer))
  (cast `/Game/Blueprint/Character/CharacterMaster` OtherActor)
  (`Widget.RemoveFromParent` (`self.WidgetRef`)))

(event `/Game/Blueprint/BPI_InteractInterface.Interact`
  (bind _result (`/Engine/EditorBlueprintResources/StandardMacros.IncrementFloat` (`self.PressedAmount`))
    (:`  `
      (bind _output_get (set `self.PressedAmount` _result))
      (`KismetSystemLibrary.K2_ClearAndInvalidateTimerHandle` (`self.TimerDecrementProgressBarRef`))
      (if (== _output_get (`self.PressesNeeded`))
        (`self.K2_DestroyActor`)
        (else
          (set `/Game/UI/SpamE/W_SpamE.AmountPressed` (stale `DecrementProgressBar` _output_get) (`self.WidgetRef`) :!label _label)
          (if (<= (`self.PressedAmount`) 0.0)
            (`KismetSystemLibrary.K2_ClearAndInvalidateTimerHandle` (`self.TimerDecrementProgressBarRef`))))))))

(event `/Game/Blueprint/BPI_InteractInterface.StopInteracting`
  (`KismetSystemLibrary.RetriggerableDelay` 0.5)
  (bind _returnvalue (`KismetSystemLibrary.K2_SetTimerDelegate` (delegate `DecrementProgressBar`) 0.2 true))
  (set `self.TimerDecrementProgressBarRef` _returnvalue))

(event `DecrementProgressBar`
  (bind _pressedamount (`self.PressedAmount`))
  (bind _result (`/Engine/EditorBlueprintResources/StandardMacros.DecrementFloat` _pressedamount)
    (:`  `
      (bind _output_get (set `self.PressedAmount` (`KismetMathLibrary.FClamp` _result 0.0 _pressedamount)))
      (goto _label))))

(fn `UserConstructionScript`)