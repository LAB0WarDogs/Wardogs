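; BP_Target is a target actor that spins around its vertical axis and plays a camera shutter sound each time it takes damage.
; It stores the root component's starting yaw on BeginPlay, then adds a timeline value scaled to 360 degrees to that yaw.
; A FlipFlop alternates successive hits between playing the timeline from the start and reversing it from the end, so the spin direction alternates.
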(event `self.ReceiveBeginPlay`
  (bind (_returnvalue_roll _returnvalue_pitch _returnvalue_yaw) (`KismetMathLibrary.BreakRotator` (`SceneComponent.K2_GetComponentRotation` (`self.DefaultSceneRoot`))))
  (bind _output_get (set `self.OriginRotation` _returnvalue_yaw)))

(event `/Game/Blueprint/BPI_Damageable.TakeDamage`
  (params (Damage :type "Float (single-precision)"))
  (bind _defaultsceneroot (`self.DefaultSceneRoot`))
  (bind (_returnvalue_roll _returnvalue_pitch _returnvalue_yaw) (`KismetMathLibrary.BreakRotator` (`SceneComponent.K2_GetComponentRotation` _defaultsceneroot)))
  (`|ExecutionSequence`
    (:`then_0`
      (`/Engine/EditorBlueprintResources/StandardMacros.FlipFlop`
        (:`A`
          (bind (_direction _newtrack_0) (`Timeline|Timeline_0` :!via `PlayFromStart` :!label _label)
            (:`Update`
              (`SceneComponent.K2_SetWorldRotation` _defaultsceneroot (`KismetMathLibrary.MakeRotator` _returnvalue_roll _returnvalue_pitch (+ (stale `self.ReceiveBeginPlay` _output_get) (* _newtrack_0 360.0))) false false))
            (:`Finished`
              (`SceneComponent.K2_SetWorldRotation` _defaultsceneroot (`KismetMathLibrary.MakeRotator` _returnvalue_roll _returnvalue_pitch _returnvalue_yaw) false false))))
        (:`B`
          (goto _label :!via `ReverseFromEnd`))))
    (:`then_1`
      (`GameplayStatics.PlaySoundAtLocation` "/Engine/VREditor/Sounds/UI/Camera_Shutter.Camera_Shutter" (`SceneComponent.K2_GetComponentLocation` _defaultsceneroot) (struct) 1.0 1.0 0.0 null null null))))

(fn `UserConstructionScript`)