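; Grenade actor that explodes three seconds after spawning, with a particle effect and sound, then hides its mesh.
; Explode runs a sphere overlap at DamageRadius, draws it as a debug sphere and sends fixed damage to BPI_Damageable actors.
; DestroyActor sits inside that loop, so the grenade is destroyed only when a damageable actor is found.
; The sphere component's overlap event is empty, and older per-character cast damage logic is left disconnected.
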(event `self.ReceiveBeginPlay`
  (`KismetSystemLibrary.Delay` 3.0)
  (`GameplayStatics.SpawnEmitterAtLocation` "/Engine/Tutorial/SubEditors/TutorialAssets/TutorialParticleSystem.TutorialParticleSystem" (`SceneComponent.K2_GetComponentLocation` (`self.Grenade`)))
  (`GameplayStatics.PlaySoundAtLocation` "/Engine/VREditor/Sounds/UI/Teleport_Committed.Teleport_Committed" (`self.K2_GetActorLocation`) (struct) 1.0 1.0 0.0 null null null)
  (`SceneComponent.SetVisibility` (`self.Grenade`) false false)
  (`self.Explode`))

(event `self.Sphere.OnComponentBeginOverlap`
  (params (OverlappedComponent :type "PrimitiveComponent Object Reference") (OtherActor :type "Actor Object Reference") (OtherComp :type "PrimitiveComponent Object Reference") (OtherBodyIndex :type Integer) (bFromSweep :type Boolean) (SweepResult :type "HitResult Structure (by ref)")))

(event `Explode`
  (bind _damageradius (`self.DamageRadius`))
  (bind _returnvalue (`SceneComponent.K2_GetComponentLocation` (`self.Grenade`)))
  (bind _outactors (`KismetSystemLibrary.SphereOverlapActors` _returnvalue _damageradius (`self.Object Types`)))
  (`KismetSystemLibrary.DrawDebugSphere` _returnvalue _damageradius 12 (struct :`R` 1.0 :`A` 1.0) 2.0)
  (for _array_element _outactors
    (if (`KismetSystemLibrary.DoesImplementInterface` _array_element "/Game/Blueprint/BPI_Damageable.BPI_Damageable_C")
      (message `/Game/Blueprint/BPI_Damageable.TakeDamage` _array_element 110.0)
      (`self.K2_DestroyActor`))))

(fn `UserConstructionScript`)