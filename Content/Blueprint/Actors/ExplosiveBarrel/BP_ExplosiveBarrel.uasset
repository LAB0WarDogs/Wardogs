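; Explosive barrel actor that BP_SecondChara can carry and set down, and that explodes when its health runs out.
; The explosion spawns an effect, hides the mesh and damages BPI_Damageable actors in a sphere; destruction follows only if one is found.
; A box overlap toggles the prompt widget and interaction.
; Interacting attaches the barrel to a character socket; stopping places it at a forward-downward trace hit, raised to offset a misplaced pivot.
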(event `self.ReceiveBeginPlay`
  (bind _returnvalue (`GameplayStatics.GetActorOfClass` "/Game/Blueprint/Character/BP_SecondChara.BP_SecondChara_C"))
  (set `self.SecondCharaRef` _returnvalue))

(event `/Game/Blueprint/BPI_Damageable.TakeDamage`
  (params (Damage :type "Float (single-precision)"))
  (bind _returnvalue (`self.K2_GetActorLocation`))
  (set `self.Health` (- (`self.Health`) Damage))
  (if (<= (`self.Health`) 0.0)
    (`NiagaraFunctionLibrary.SpawnSystemAtLocation` null (`self.K2_GetActorLocation`))
    (`SceneComponent.SetVisibility` (`self.Cylinder`) false false)
    (bind _outactors (`KismetSystemLibrary.SphereOverlapActors` _returnvalue (`self.Sphere Radius`) (`self.Object Types`) null (`|MakeArray` self :!type "Actor Object Reference")))
    (`KismetSystemLibrary.DrawDebugSphere` _returnvalue (`self.Sphere Radius`) 12 (struct :`R` 1.0 :`G` 1.0 :`B` 1.0 :`A` 1.0) 1.0)
    (for _array_element _outactors
      (if (`KismetSystemLibrary.DoesImplementInterface` _array_element "/Game/Blueprint/BPI_Damageable.BPI_Damageable_C")
        (message `/Game/Blueprint/BPI_Damageable.TakeDamage` _array_element 110.0)
        (message `/Game/Blueprint/BPI_Damageable.EnvironmentTakingDamage` _array_element 110.0)
        (`KismetSystemLibrary.Delay` 0.1)
        (`self.K2_DestroyActor`)))))

(event `/Game/Blueprint/BPI_InteractInterface.Interact`
  (bind _secondchararef (`self.SecondCharaRef`))
  (if (and (not (`self.IsAttached`)) (`self.CanInteract`))
    (`/Engine/EditorBlueprintResources/StandardMacros.IsValid` _secondchararef
      (:`Is Valid`
        (`self.K2_AttachToComponent` (`Character.Mesh` _secondchararef) "BarilsSocket" "SnapToTarget" "SnapToTarget" "SnapToTarget")
        (`SceneComponent.SetHiddenInGame` (`self.Widget`) true false)
        (`KismetSystemLibrary.Delay` 1.0)
        (set `self.IsAttached` true)))))

(event `/Game/Blueprint/BPI_InteractInterface.StopInteracting`
  (if (`self.IsAttached`)
    (bind _outhit (`KismetSystemLibrary.LineTraceSingle` :`Start` (`self.K2_GetActorLocation` (`self.SecondCharaRef`)) :`End` (+ (- (`self.K2_GetActorLocation` (`self.SecondCharaRef`)) (0.0 0.0 500.0)) (* (`self.GetActorForwardVector` (`self.SecondCharaRef`)) 500.0)) :`TraceChannel` "TraceTypeQuery1" :`DrawDebugType` "ForDuration"))
    (`self.K2_DetachFromActor` self "KeepWorld" "KeepWorld" "KeepWorld")
    (bind (_bblockinghit _binitialoverlap _time _distance _location _impactpoint) (`GameplayStatics.BreakHitResult` _outhit))
    (`self.K2_SetActorTransform` self (`KismetMathLibrary.MakeTransform` (`KismetMathLibrary.MakeVector` (.x _impactpoint) (.y _impactpoint) (+ (.z _impactpoint) 50.0))) false false)
    (`SceneComponent.SetHiddenInGame` (`self.Widget`) false false)
    (set `self.IsAttached` false)))

(event `self.Box.OnComponentBeginOverlap`
  (params (OverlappedComponent :type "PrimitiveComponent Object Reference") (OtherActor :type "Actor Object Reference") (OtherComp :type "PrimitiveComponent Object Reference") (OtherBodyIndex :type Integer) (bFromSweep :type Boolean) (SweepResult :type "HitResult Structure (by ref)"))
  (cast `/Game/Blueprint/Character/BP_SecondChara` OtherActor)
  (`SceneComponent.SetVisibility` (`self.Widget`) true false)
  (set `self.CanInteract` true))

(event `self.Box.OnComponentEndOverlap`
  (params (OverlappedComponent :type "PrimitiveComponent Object Reference") (OtherActor :type "Actor Object Reference") (OtherComp :type "PrimitiveComponent Object Reference") (OtherBodyIndex :type Integer))
  (cast `/Game/Blueprint/Character/BP_SecondChara` OtherActor)
  (`SceneComponent.SetVisibility` (`self.Widget`) false false)
  (set `self.CanInteract` false))

(fn `UserConstructionScript`)