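; BP_DissolveMask is an actor that hovers above the active character and drives the area used for a dissolve effect.
; It starts on BP_FirstChara and retargets through a game mode event when the player switches characters.
; A fast looping timer moves it over the target and writes its mesh location and scale to the MPC_DIssolveArea material parameter collection.
; The construction script writes the same parameters, so the area also updates in the editor.
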(event `self.ReceiveBeginPlay`
  (`|ExecutionSequence`
    (:`then_0`
      (bind _returnvalue (`GameplayStatics.GetActorOfClass` "/Game/Blueprint/Character/BP_FirstChara.BP_FirstChara_C"))
      (set `self.ActorToFollow` _returnvalue))
    (:`then_1`
      (bind _asgame_mode_wardogs (`/Game/Blueprint/FL_Main.GetGameMode`))
      (add `/Game/Blueprint/GameMode/GameModeWardogs.CharacterAsBeenSwitched` _asgame_mode_wardogs (delegate `OnCharacterSwitch`)))
    (:`then_2`
      (`KismetSystemLibrary.K2_SetTimerDelegate` (delegate `SetPosAndVectorValue`) 0.02 true))))

(event `OnCharacterSwitch`
  (bind _asgame_mode_wardogs (`/Game/Blueprint/FL_Main.GetGameMode`))
  (bind _output_get (set `self.ActorToFollow` (`|GetArrayItem` (`/Game/Blueprint/GameMode/GameModeWardogs.ArrayCharaRef` _asgame_mode_wardogs) (`/Game/Blueprint/GameMode/GameModeWardogs.CharaIndex` (stale `self.ReceiveBeginPlay` _asgame_mode_wardogs)))))
  (`KismetSystemLibrary.PrintString` (`KismetStringLibrary.Concat_StrStr` (`KismetSystemLibrary.GetDisplayName` _output_get) " is being followed by Dissolved Masked")))

(event `SetPosAndVectorValue`
  (bind _staticmesh (`self.StaticMesh`))
  (bind _actortofollow (`self.ActorToFollow`)
    (:`then`
      (bind (_returnvalue_x _returnvalue_y _returnvalue_z) (`KismetMathLibrary.BreakVector` (`self.K2_GetActorLocation` _actortofollow)))
      (`self.K2_SetActorLocation` (`KismetMathLibrary.MakeVector` _returnvalue_x _returnvalue_y (+ _returnvalue_z 300.0)))
      (`KismetMaterialLibrary.SetVectorParameterValue` "/Game/Material/DissolveMask/MPC_DIssolveArea.MPC_DIssolveArea" "Location" (`KismetMathLibrary.Conv_VectorToLinearColor` (`SceneComponent.K2_GetComponentLocation` _staticmesh)))
      (`KismetMaterialLibrary.SetVectorParameterValue` "/Game/Material/DissolveMask/MPC_DIssolveArea.MPC_DIssolveArea" "Scale" (`KismetMathLibrary.Conv_VectorToLinearColor` (`SceneComponent.K2_GetComponentScale` _staticmesh))))
    (:`else`)))

(fn `UserConstructionScript`
  (bind _staticmesh (`self.StaticMesh`))
  (`KismetMaterialLibrary.SetVectorParameterValue` "/Game/Material/DissolveMask/MPC_DIssolveArea.MPC_DIssolveArea" "Location" (`KismetMathLibrary.Conv_VectorToLinearColor` (`SceneComponent.K2_GetComponentLocation` _staticmesh)))
  (`KismetMaterialLibrary.SetVectorParameterValue` "/Game/Material/DissolveMask/MPC_DIssolveArea.MPC_DIssolveArea" "Scale" (`KismetMathLibrary.Conv_VectorToLinearColor` (`SceneComponent.K2_GetComponentScale` _staticmesh))))