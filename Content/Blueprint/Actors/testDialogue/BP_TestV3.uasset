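; BP_TestV3 is a test dialogue NPC, controlled by a BP_Test_AI controller, that starts a conversation when a Character overlaps it.
; On BeginPlay it passes its dialogue tree to that AI controller and hides its widget.
; On overlap it calls StartDialogue on the controller, which handles the dialogue itself.
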(event `self.ReceiveBeginPlay`
  ;[0 1 0] Set Tree used
  (bind _asbp_test_ai (cast `/Game/Blueprint/Actors/testDialogue/BP_Test_AI` (`AIBlueprintHelperLibrary.GetAIController` self)))
  (set `/Game/Blueprint/Actors/testDialogue/BP_Test_AI.DialogueTree` (`self.DialogeTree`) _asbp_test_ai)
  (`SceneComponent.SetVisibility` (`self.Widget`) false false))

(event `self.ReceiveActorBeginOverlap`
  (params (OtherActor :type "Actor Object Reference"))
  ;[0 1 0] Interact
  (cast `Character` OtherActor)
  (bind _asbp_test_ai (cast `/Game/Blueprint/Actors/testDialogue/BP_Test_AI` (`AIBlueprintHelperLibrary.GetAIController` self)))
  (`/Game/Blueprint/Actors/testDialogue/BP_Test_AI.StartDialogue` _asbp_test_ai))

(fn `UserConstructionScript`)