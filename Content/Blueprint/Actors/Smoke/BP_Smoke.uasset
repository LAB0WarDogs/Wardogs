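; BP_Smoke is a timed actor that turns from a placeholder sphere into a collidable static mesh, then removes itself.
; On BeginPlay it disables mesh collision and waits a short fixed delay.
; It then plays the Teleport_Committed sound, hides the sphere with its children, and shows the mesh with query and physics collision.
; After a further LifeTime delay, the actor destroys itself.
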(event `self.ReceiveBeginPlay`
  (bind _staticmesh (`self.StaticMesh`))
  (`PrimitiveComponent.SetCollisionEnabled` (`self.StaticMesh`) "NoCollision")
  (`KismetSystemLibrary.Delay` 2.5)
  (`GameplayStatics.PlaySoundAtLocation` "/Engine/VREditor/Sounds/UI/Teleport_Committed.Teleport_Committed" (`self.K2_GetActorLocation`) (struct) 1.0 1.0 0.0 null null null)
  (`SceneComponent.SetVisibility` (`self.Sphere`) false true)
  (`PrimitiveComponent.SetCollisionEnabled` _staticmesh "QueryAndPhysics")
  (`SceneComponent.SetVisibility` _staticmesh true true)
  (`KismetSystemLibrary.Delay` (`self.LifeTime`))
  (`self.K2_DestroyActor`))

(fn `UserConstructionScript`)