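; BP_SightLine is an actor that follows the active character and builds a line-of-sight mask around it.
; Each tick it fires a ring of visibility traces and scales one instanced mesh wedge per ray to the hit distance.
; An orthographic scene capture is sized to the check range, and a material parameter collection receives position, height and scale for materials.
; A game mode event retargets it when the character switches.
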(event `self.ReceiveBeginPlay`
  (`|ExecutionSequence`
    (:`then_0`
      (`self.InitialiaseISM`)
      (bind _outactors (`GameplayStatics.GetAllActorsOfClass` (`self.ClassToFollow`)))
      (set `self.ActorToFollow` (`|GetArrayItem` _outactors)))
    (:`then_1`
      (bind _asgame_mode_wardogs (`/Game/Blueprint/FL_Main.GetGameMode`))
      (add `/Game/Blueprint/GameMode/GameModeWardogs.CharacterAsBeenSwitched` _asgame_mode_wardogs (delegate `OnCharacterSwitch`)))))

(event `OnCharacterSwitch`
  (bind _outactors (`GameplayStatics.GetAllActorsOfClass` (`self.ClassToFollow`)))
  (set `self.ActorToFollow` (`|GetArrayItem` _outactors (`/Game/Blueprint/GameMode/GameModeWardogs.CharaIndex` (stale `self.ReceiveBeginPlay` _asgame_mode_wardogs)))))

(event `self.ReceiveTick`
  (params (DeltaSeconds :type "Float (single-precision)"))
  (bind _actortofollow (`self.ActorToFollow`)
    (:`then`
      (`self.K2_SetActorLocation` (`self.K2_GetActorLocation` _actortofollow))
      (`self.SightTrace`)
      (`KismetMaterialLibrary.SetVectorParameterValue` "/Game/Blueprint/SightLine/MPC_SightLIne.MPC_SightLIne" "SightLineActorLocation" (`KismetMathLibrary.Conv_VectorToLinearColor` (`self.K2_GetActorLocation`))))
    (:`else`)))

(fn `InitialiaseISM`
  (bind (_returnvalue_x _returnvalue_y _returnvalue_z) (`KismetMathLibrary.BreakVector` (`self.K2_GetActorLocation`)))
  (`InstancedStaticMeshComponent.ClearInstances` (`self.InstancedStaticMesh`))
  (for _ (range (`self.TraceCount`))
    (`InstancedStaticMeshComponent.AddInstance` (`self.InstancedStaticMesh`) (`KismetMathLibrary.MakeTransform` (0.0 0.0 0.0))))
  (`self.SightTrace`)
  (set `SceneCaptureComponent2D.OrthoWidth` (`self.CheckRange`) (`self.SceneCaptureComponent2D`))
  (`SceneComponent.K2_SetRelativeTransform` (`self.SceneCaptureComponent2D`) (`KismetMathLibrary.MakeTransform` (`KismetMathLibrary.MakeVector` 0.0 0.0 (- (`self.ISM_HeightOffset`) 1.0)) (struct :`Pitch` 90.0) (1.0 -1.0 -1.0)) false false)
  (`KismetMaterialLibrary.SetScalarParameterValue` "/Game/Blueprint/SightLine/MPC_SightLIne.MPC_SightLIne" "SightLineMaskHeight" (+ _returnvalue_z (`self.ISM_HeightOffset`) -500.0))
  (`KismetMaterialLibrary.SetScalarParameterValue` "/Game/Blueprint/SightLine/MPC_SightLIne.MPC_SightLIne" "SightLineTexScale" (`self.CheckRange`))
  (`KismetMaterialLibrary.SetVectorParameterValue` "/Game/Blueprint/SightLine/MPC_SightLIne.MPC_SightLIne" "SightLineActorLocation" (`KismetMathLibrary.Conv_VectorToLinearColor` (`self.K2_GetActorLocation`))))

(fn `SightTrace`
  (bind _returnvalue (`self.K2_GetActorLocation`))
  (for _index (range (`self.TraceCount`))
    (bind _output_get (set `self.CurrentTraceStep` _index))
    (bind (_outhit _returnvalue_2) (`KismetSystemLibrary.LineTraceSingle` :`Start` _returnvalue :`End` (+ _returnvalue (* (`KismetMathLibrary.GreaterGreater_VectorRotator` (`self.GetActorForwardVector`) (`KismetMathLibrary.MakeRotator` 0.0 0.0 (* (`KismetMathLibrary.Conv_IntToDouble` _output_get) (/ 360.0 (`KismetMathLibrary.Conv_IntToDouble` (`self.TraceCount`)))))) (`self.CheckRange`))) :`TraceChannel` "TraceTypeQuery1" :`DrawTime` 0.1))
    (bind (_bblockinghit _binitialoverlap _time _distance _location _impactpoint _normal _impactnormal _physmat _hitactor _hitcomponent _hitbonename _hititem _elementindex _faceindex _tracestart _traceend) (`GameplayStatics.BreakHitResult` _outhit))
    (bind _returnvalue_3 (* (`KismetMathLibrary.VSize` (- (`KismetMathLibrary.SelectVector` _location _traceend _returnvalue_2) _tracestart)) (`self.TraceHitOffset`)))
    (`InstancedStaticMeshComponent.UpdateInstanceTransform` (`self.InstancedStaticMesh`) (`self.CurrentTraceStep`) (`KismetMathLibrary.MakeTransform` (`KismetMathLibrary.SelectVector` (`KismetMathLibrary.MakeVector` 0.0 0.0 (`self.ISM_HeightOffset`)) (0.0 0.0 0.0) (`self.OffsetByHeight`)) (`KismetMathLibrary.FindLookAtRotation` _tracestart _traceend) (`KismetMathLibrary.MakeVector` _returnvalue_3 (* (/ 360.0 (`KismetMathLibrary.Conv_IntToDouble` (`self.TraceCount`))) _returnvalue_3) _returnvalue_3)) false true true)))

(fn `UserConstructionScript`
  (`self.InitialiaseISM`))