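; BP_RtsCamera is an RTS camera rig with events for panning, turning, tilting and zooming.
; Axis values scaled by speed variables move the actor along its local X and Y and yaw it, so panning follows the camera's heading.
; Tilt rotates the SpringArm and clamps its pitch to a downward range.
; Zoom and dezoom change the arm length in fixed, unclamped steps; movement is neither swept nor delta-time scaled.
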(event `RtsHorizontalMovement`
  (params (AxisValue :type "Float (double-precision)"))
  (`self.K2_AddActorLocalOffset` (`KismetMathLibrary.MakeVector` 0.0 (* AxisValue (`self.MoveSpeed`)))))

(event `TurnRtsCamera`
  (params (AxisValue :type "Float (double-precision)"))
  (`self.K2_AddActorLocalRotation` (`KismetMathLibrary.MakeRotator` 0.0 0.0 (* AxisValue (`self.TurnSpeed`)))))

(event `RtsVerticalMovement`
  (params (AxisValue :type "Float (double-precision)"))
  (`self.K2_AddActorLocalOffset` (`KismetMathLibrary.MakeVector` (* AxisValue (`self.MoveSpeed`)))))

(event `ChangeRtsCamAngle`
  (params (AxisValue :type "Float (double-precision)"))
  (bind (_returnvalue_location _returnvalue_rotation) (`KismetMathLibrary.BreakTransform` (`SceneComponent.GetRelativeTransform` (`self.SpringArm`))))
  (`SceneComponent.K2_AddRelativeRotation` (`self.SpringArm`) (`KismetMathLibrary.MakeRotator` 0.0 (* AxisValue (`self.AngleSpeed`))) false false)
  (`SceneComponent.K2_SetRelativeRotation` (`self.SpringArm`) (`KismetMathLibrary.MakeRotator` 0.0 (`KismetMathLibrary.FClamp` (.pitch _returnvalue_rotation) -80.0 -30.0)) false false))

(event `Zoom`
  (bind _springarm (`self.SpringArm`))
  (set `SpringArmComponent.TargetArmLength` (- (`SpringArmComponent.TargetArmLength` _springarm) 50.0) _springarm))

(event `dezoom`
  (bind _springarm (`self.SpringArm`))
  (set `SpringArmComponent.TargetArmLength` (+ (`SpringArmComponent.TargetArmLength` _springarm) 50.0) _springarm))

(fn `UserConstructionScript`)