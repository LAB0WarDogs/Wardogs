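; Behavior Tree task that starts a dialogue by switching the HUD into dialogue display.
; Its Cinematique flag, copied to the blackboard, picks either a mid-screen box with player input disabled or a top-screen box with an icon border.
; It stores the chosen widget in the blackboard, hides and disables the in-game UI, then finishes successfully.
; A failed GameModeWardogs cast leaves the task unfinished.
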(event `self.ReceiveExecuteAI`
  (params (OwnerController :type "AIController Object Reference") (ControlledPawn :type "Pawn Object Reference"))
  (bind _returnvalue (`GameplayStatics.GetPlayerController` 0))
  (bind _cinematique (`self.Cinematique`))
  ;[0 1 0] Start Dialogue System
  (bind _asgame_mode_wardogs (cast `/Game/Blueprint/GameMode/GameModeWardogs` (`GameplayStatics.GetGameMode`)))
  (`BTFunctionLibrary.SetBlackboardValueAsBool` (`self.BB_Cinematique`) _cinematique)
  ;;[0 0 0] Text in Mid Screen
  (if _cinematique
    (bind _headupdisplay (`/Game/Blueprint/GameMode/GameModeWardogs.HeadUpDisplay` _asgame_mode_wardogs))
    (bind _dialoguebox_40 (`/Game/UI/Dialogue/HeadUpDisplay.DialogueBox_40` _headupdisplay))
    (`Widget.SetVisibility` _dialoguebox_40 "Visible")
    (`BTFunctionLibrary.SetBlackboardValueAsObject` (`self.BB_DialogueUI`) _dialoguebox_40)
    (`Actor.DisableInput` _returnvalue _returnvalue)
    (else
      (bind _dialoguebox (`/Game/UI/Dialogue/HeadUpDisplay.DialogueBox` _headupdisplay))
      ;;[0 0 0] Text in Top Screen
      (`Widget.SetVisibility` _dialoguebox "Visible")
      (`Widget.SetVisibility` (`/Game/UI/Dialogue/DialogueBox.BorderIcone` _dialoguebox) "Visible")
      (`BTFunctionLibrary.SetBlackboardValueAsObject` (`self.BB_DialogueUI`) _dialoguebox)))
  (bind _asgame_mode_wardogs_2 (`/Game/Blueprint/FL_Main.GetGameMode`))
  (bind _ingameui (`/Game/Blueprint/GameMode/GameModeWardogs.InGameUI` _asgame_mode_wardogs_2))
  (`Widget.SetIsEnabled` _ingameui false)
  (`Widget.SetVisibility` _ingameui "Hidden")
  (`self.FinishExecute` true))