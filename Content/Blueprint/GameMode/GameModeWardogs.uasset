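; Game mode for Wardogs that lets the player switch between three characters and shows the end screen when two or fewer remain.
; BeginPlay registers the characters, creates the HUD widgets and starts a looping timer that checks the remaining count.
; Switching cycles the array index, cancels every character's action and updates the UI.
; PossesChara blends the camera with input disabled, then possesses the new pawn and respawns the previous one's default controller.
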(event `SwitchChara0`
  ;[0 0 1] Switch Character
  (if (and (`self.CanSwitch`) (`self.IsSwitching`))
    (bind _ascharacter_master (cast `/Game/Blueprint/Character/CharacterMaster` (`GameplayStatics.GetPlayerCharacter` 0)))
    (set `self.camRotate` (`/Game/Blueprint/Character/CharacterMaster.CamRotation` _ascharacter_master))
    (`|ExecutionSequence`
      (:`then_0`
        (bind _output_get (set `self.CharaIndex` (+ (`self.CharaIndex`) 1)))
        (if (> _output_get (- (`KismetArrayLibrary.Array_Length` (`self.ArrayCharaRef`)) 1))
          (set `self.CharaIndex` 0))
        (bind _aspawn (cast `Pawn` (`|GetArrayItem` (`self.ArrayCharaRef`) (`self.CharaIndex`))))
        (`self.PossesChara` _aspawn)
        (`self.CharacterAsBeenSwitched`)
        ;[0 1 0] Call Ui SwhichChara
        (`/Game/UI/UI_InGame/Widget_HeadUp.Switch` (`self.InGameUI`) (`self.CharaIndex`) :!label _label)
        (set `self.IsSwitching` false))
      (:`then_1`
        (for _array_element (`self.ArrayCharaRef`)
          (bind _ascharacter_master_2 (cast `/Game/Blueprint/Character/CharacterMaster` _array_element))
          (`/Game/Blueprint/Character/CharacterMaster.CancelAction` _ascharacter_master_2))))))

(event `SwitchChara1`
  ;[0 0 1] Switch Character
  (if (and (`self.CanSwitch`) (`self.IsSwitching`))
    (bind _ascharacter_master (cast `/Game/Blueprint/Character/CharacterMaster` (`GameplayStatics.GetPlayerCharacter` 0)))
    (set `self.camRotate` (`/Game/Blueprint/Character/CharacterMaster.CamRotation` _ascharacter_master))
    (`|ExecutionSequence`
      (:`then_0`
        (bind _output_get (set `self.CharaIndex` (- (`self.CharaIndex`) 1)))
        (if (< _output_get 0)
          (set `self.CharaIndex` (- (`KismetArrayLibrary.Array_Length` (`self.ArrayCharaRef`)) 1)))
        (bind _aspawn (cast `Pawn` (`|GetArrayItem` (`self.ArrayCharaRef`) (`self.CharaIndex`))))
        (`self.PossesChara` _aspawn)
        (`self.CharacterAsBeenSwitched`)
        (goto _label))
      (:`then_1`
        (for _array_element (`self.ArrayCharaRef`)
          (bind _ascharacter_master_2 (cast `/Game/Blueprint/Character/CharacterMaster` _array_element))
          (`/Game/Blueprint/Character/CharacterMaster.CancelAction` _ascharacter_master_2))))))

(event `self.ReceiveBeginPlay`
  ;[0 0 1] Begin Play
  (`|ExecutionSequence`
    (:`then_0`
      (bind _returnvalue (`GameplayStatics.GetActorOfClass` "/Game/Blueprint/Character/BP_FirstChara.BP_FirstChara_C"))
      (`KismetArrayLibrary.Array_Add` (`self.ArrayCharaRef`) _returnvalue))
    (:`then_1`
      (bind _returnvalue_2 (`GameplayStatics.GetActorOfClass` "/Game/Blueprint/Character/BP_SecondChara.BP_SecondChara_C"))
      (`KismetArrayLibrary.Array_Add` (`self.ArrayCharaRef`) _returnvalue_2))
    (:`then_2`
      (bind _returnvalue_3 (`GameplayStatics.GetActorOfClass` "/Game/Blueprint/Character/BP_ThirdChara.BP_ThirdChara_C"))
      (`KismetArrayLibrary.Array_Add` (`self.ArrayCharaRef`) _returnvalue_3)
      (bind _output_get (set `self.LastPlayerSelected` (`|GetArrayItem` (`self.ArrayCharaRef`))))
      (`KismetSystemLibrary.PrintString` (`KismetSystemLibrary.GetDisplayName` _output_get)))
    (:`then_3`
      ;;[0 1 0] Set HeadUpDisplay
      (bind _returnvalue_4 (`|CreateWidget` "/Game/UI/Dialogue/HeadUpDisplay.HeadUpDisplay_C"))
      (bind _output_get_2 (set `self.HeadUpDisplay` _returnvalue_4))
      (`UserWidget.AddToViewport` _output_get_2 0)
      (bind _returnvalue_5 (`|CreateWidget` "/Game/UI/UI_InGame/Widget_HeadUp.Widget_HeadUp_C"))
      (bind _output_get_3 (set `self.InGameUI` _returnvalue_5))
      (`UserWidget.AddToViewport` _output_get_3 0))
    (:`then_4`
      (`KismetSystemLibrary.K2_SetTimerDelegate` (delegate `ResetScene`) 0.5 true))))

(event `ResetScene`
  (bind _returnvalue (`GameplayStatics.GetPlayerController` 0))
  ;[0 0 1] Begin Play
  (if (<= (`KismetArrayLibrary.Array_Length` (`self.ArrayCharaRef`)) 2)
    (`/Engine/EditorBlueprintResources/StandardMacros.DoOnce` false
      (:`Completed`
        (bind _returnvalue_2 (`|CreateWidget` "/Game/UI/UI_Unique/W_EndGame.W_EndGame_C"))
        (`UserWidget.AddToViewport` _returnvalue_2 0)
        (set `PlayerController.bShowMouseCursor` true _returnvalue)
        (`WidgetBlueprintLibrary.SetInputMode_UIOnlyEx` _returnvalue null)))))

(event `RemoveFromPlayerList`
  (params (CharaRef :type "Actor Object Reference"))
  (bind _arraychararef (`self.ArrayCharaRef`))
  ;[0 0 1] Remove From Player List
  (`KismetArrayLibrary.Array_RemoveItem` _arraychararef CharaRef)
  (`KismetSystemLibrary.PrintString` (`KismetStringLibrary.Concat_StrStr` "number of player left " (`KismetStringLibrary.Conv_IntToString` (`KismetArrayLibrary.Array_Length` _arraychararef)))))

(fn `UserConstructionScript`)