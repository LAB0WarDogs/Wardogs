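; BP_GrapplingHook is an interactable grapple point that pulls the first character (BP_FirstChara, noted as the Genie) to a set end point.
; A Box overlap shows or hides a prompt widget only for that character.
; On Interact, it passes the player's current location and the GrappleEnd component's location to the character, calls its MovePlayerAlongGrapple, and hides the widget.
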(event `/Game/Blueprint/BPI_InteractInterface.Interact`
  ;[0 0 1] Only the Genie will be able to use grappling hook
  (bind _asbp_first_chara (cast `/Game/Blueprint/Character/BP_FirstChara` (`GameplayStatics.GetPlayerCharacter` 0)))
  (set `/Game/Blueprint/Character/BP_FirstChara.GrappleStartLocation` (`self.K2_GetActorLocation` _asbp_first_chara) _asbp_first_chara)
  (set `/Game/Blueprint/Character/BP_FirstChara.GrappleEndLocation` (`SceneComponent.K2_GetComponentLocation` (`self.GrappleEnd`)) _asbp_first_chara)
  (`/Game/Blueprint/Character/BP_FirstChara.MovePlayerAlongGrapple` _asbp_first_chara)
  (`SceneComponent.SetVisibility` (`self.Widget`) false false))

(event `self.Box.OnComponentBeginOverlap`
  (params (OverlappedComponent :type "PrimitiveComponent Object Reference") (OtherActor :type "Actor Object Reference") (OtherComp :type "PrimitiveComponent Object Reference") (OtherBodyIndex :type Integer) (bFromSweep :type Boolean) (SweepResult :type "HitResult Structure (by ref)"))
  (cast `/Game/Blueprint/Character/BP_FirstChara` OtherActor)
  (`SceneComponent.SetVisibility` (`self.Widget`) true false))

(event `self.Box.OnComponentEndOverlap`
  (params (OverlappedComponent :type "PrimitiveComponent Object Reference") (OtherActor :type "Actor Object Reference") (OtherComp :type "PrimitiveComponent Object Reference") (OtherBodyIndex :type Integer))
  (cast `/Game/Blueprint/Character/BP_FirstChara` OtherActor)
  (`SceneComponent.SetVisibility` (`self.Widget`) false false))

(fn `UserConstructionScript`)