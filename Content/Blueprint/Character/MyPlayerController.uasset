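; Player controller that routes input to the current CharacterMaster for movement, look, sprint, sneak, skills, interaction and regroup/separate, and asks the GameMode to switch between two characters.
; It caches the HeadUp widget at BeginPlay; during its QTE, movement axes become directional inputs and skills and switching are blocked.
; IsBeingAttack blocks most actions and redirects Interact to enemy interaction.
; A temporary P key reloads the level for the training room.
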(event `InputAxis|MouseLookHorizontal`
  (params (AxisValue :type "Float (single-precision)"))
  ;[0 0 1] Look horizontal
  (bind _ascharacter_master (`/Game/Blueprint/FL_Main.Get Player Character Master`))
  (`/Engine/EditorBlueprintResources/StandardMacros.IsValid` _ascharacter_master
    (:`Is Valid`
      (`/Game/Blueprint/Character/CharacterMaster.HorizontalLook` _ascharacter_master AxisValue))))

(event `self.ReceiveTick`
  (params (DeltaSeconds :type "Float (single-precision)"))
  ;[0 0 1] Event Tick For Gamepad Control
  (set `self.JoystickX` (`self.GetInputAxisKeyValue`))
  (set `self.JoystickY` (`self.GetInputAxisKeyValue`)))

(event `self.ReceiveBeginPlay`
  ;[0 0 1] Begin Play
  (`|ExecutionSequence`
    (:`then_0`
      (bind _foundwidgets (`WidgetBlueprintLibrary.GetAllWidgetsOfClass` "/Game/UI/UI_InGame/Widget_HeadUp.Widget_HeadUp_C"))
      (set `self.In Game UI` (`|GetArrayItem` _foundwidgets)))))

(event `Key|P`
  (params (Key :type "Key Structure"))
  ;[1 0 0] Training Room uniquement a degager après
  (:`Pressed`
    (bind _returnvalue (`GameplayStatics.GetCurrentLevelName` true))
    (`GameplayStatics.OpenLevel` (`KismetStringLibrary.Conv_StringToName` _returnvalue))))

(event `InputAction|SwitchToChara1`
  (params (Key :type "Key Structure"))
  ;[0 0 1] Switch character
  (:`Pressed`
    (if (not (`/Game/UI/UI_InGame/Widget_HeadUp.InQTE` (`self.In Game UI`)))
      (bind _asgame_mode_wardogs (`/Game/Blueprint/FL_Main.GetGameMode`))
      (if (not (`/Game/Blueprint/GameMode/GameModeWardogs.IsSwitching` _asgame_mode_wardogs))
        (set `/Game/Blueprint/GameMode/GameModeWardogs.IsSwitching` true _asgame_mode_wardogs)
        (bind _asgame_mode_wardogs_2 (`/Game/Blueprint/FL_Main.GetGameMode`))
        (`/Game/Blueprint/GameMode/GameModeWardogs.SwitchChara0` _asgame_mode_wardogs_2)))))

(event `InputAction|SwitchToChara2`
  (params (Key :type "Key Structure"))
  ;[0 0 1] Switch character
  (:`Pressed`
    (if (not (`/Game/UI/UI_InGame/Widget_HeadUp.InQTE` (`self.In Game UI`)))
      (bind _asgame_mode_wardogs (`/Game/Blueprint/FL_Main.GetGameMode`))
      (if (not (`/Game/Blueprint/GameMode/GameModeWardogs.IsSwitching` _asgame_mode_wardogs))
        (set `/Game/Blueprint/GameMode/GameModeWardogs.IsSwitching` true _asgame_mode_wardogs)
        (bind _asgame_mode_wardogs_2 (`/Game/Blueprint/FL_Main.GetGameMode`))
        (`/Game/Blueprint/GameMode/GameModeWardogs.SwitchChara1` _asgame_mode_wardogs_2)))))

(event `InputAxis|Horizontal`
  (params (AxisValue :type "Float (single-precision)"))
  (bind _in_game_ui (`self.In Game UI`))
  (bind _in_game_ui_2 (`self.In Game UI`))
  ;[0 0 1] Movement Horizontal Axis
  (if (`/Game/UI/UI_InGame/Widget_HeadUp.InQTE` (`self.In Game UI`))
    (if (> AxisValue 0.0)
      (`/Engine/EditorBlueprintResources/StandardMacros.IsValid` _in_game_ui
        (:`Is Valid`
          (`/Game/UI/UI_InGame/Widget_HeadUp.EnterInput` _in_game_ui 4)))
      (elif (< AxisValue 0.0)
        (`/Engine/EditorBlueprintResources/StandardMacros.IsValid` _in_game_ui_2
          (:`Is Valid`
            (`/Game/UI/UI_InGame/Widget_HeadUp.EnterInput` _in_game_ui_2 2)))))
    (else
      (bind _ascharacter_master (`/Game/Blueprint/FL_Main.Get Player Character Master`))
      (`/Engine/EditorBlueprintResources/StandardMacros.IsValid` _ascharacter_master
        (:`Is Valid`
          (`/Game/Blueprint/Character/CharacterMaster.HorizontalMovement` _ascharacter_master AxisValue))))))

(event `InputAction|sprint`
  (params (Key :type "Key Structure"))
  ;[0 0 1] Sprint
  (:`Pressed`
    (bind _ascharacter_master (`/Game/Blueprint/FL_Main.Get Player Character Master`))
    (`/Engine/EditorBlueprintResources/StandardMacros.IsValid` _ascharacter_master
      (:`Is Valid`
        (`/Game/Blueprint/Character/CharacterMaster.Sprint` _ascharacter_master))))
  (:`Released`
    (bind _ascharacter_master_2 (`/Game/Blueprint/FL_Main.Get Player Character Master`))
    (`/Engine/EditorBlueprintResources/StandardMacros.IsValid` _ascharacter_master_2
      (:`Is Valid`
        (`/Game/Blueprint/Character/CharacterMaster.Walk` _ascharacter_master_2)))))

(event `InputAction|Sneak`
  (params (Key :type "Key Structure"))
  ;[0 0 1] Sneak
  (:`Pressed`
    (if (not (`self.IsBeingAttack`))
      (bind _ascharacter_master (`/Game/Blueprint/FL_Main.Get Player Character Master`))
      (`/Engine/EditorBlueprintResources/StandardMacros.IsValid` _ascharacter_master
        (:`Is Valid`
          (`/Game/Blueprint/Character/CharacterMaster.Sneak` _ascharacter_master)))))
  (:`Released`
    (if (not (`self.IsBeingAttack`))
      (bind _ascharacter_master_2 (`/Game/Blueprint/FL_Main.Get Player Character Master`))
      (`/Engine/EditorBlueprintResources/StandardMacros.IsValid` _ascharacter_master_2
        (:`Is Valid`
          (`/Game/Blueprint/Character/CharacterMaster.StopSneaking` _ascharacter_master_2))))))

(event `InputAction|CancelAction`
  (params (Key :type "Key Structure"))
  ;[0 0 1] Cancel Action/Skills
  (:`Pressed`
    (if (not (`self.IsBeingAttack`))
      (bind _ascharacter_master (`/Game/Blueprint/FL_Main.Get Player Character Master`))
      (`/Game/Blueprint/Character/CharacterMaster.CancelAction` _ascharacter_master))))

(event `InputAction|PrimarySkill`
  (params (Key :type "Key Structure"))
  ;[0 0 1] Skills
  (:`Pressed`
    (if (not (`/Game/UI/UI_InGame/Widget_HeadUp.InQTE` (`self.In Game UI`)))
      (if (not (`self.IsBeingAttack`))
        (bind _ascharacter_master (`/Game/Blueprint/FL_Main.Get Player Character Master`))
        (`/Game/Blueprint/Character/CharacterMaster.primarySkillActivation` _ascharacter_master)))))

(event `InputAction|Regroup`
  (params (Key :type "Key Structure"))
  ;[0 0 1] Regroup / Separate
  (:`Pressed`
    (if (not (`self.IsBeingAttack`))
      (bind _ascharacter_master (`/Game/Blueprint/FL_Main.Get Player Character Master`))
      (`/Game/Blueprint/Character/CharacterMaster.Regroup` _ascharacter_master))))

(event `InputAction|SecondSKill`
  (params (Key :type "Key Structure"))
  ;[0 0 1] Skills
  (:`Pressed`
    (if (not (`/Game/UI/UI_InGame/Widget_HeadUp.InQTE` (`self.In Game UI`)))
      (if (not (`self.IsBeingAttack`))
        (bind _ascharacter_master (`/Game/Blueprint/FL_Main.Get Player Character Master`))
        (`/Game/Blueprint/Character/CharacterMaster.SecondarySkillActivation` _ascharacter_master)))))

(event `InputAction|Interact`
  (params (Key :type "Key Structure"))
  ;[0 0 1] Interact
  (:`Pressed`
    (if (not (`self.IsBeingAttack`))
      (bind _ascharacter_master (`/Game/Blueprint/FL_Main.Get Player Character Master`))
      (`/Engine/EditorBlueprintResources/StandardMacros.IsValid` _ascharacter_master
        (:`Is Valid`
          (`/Game/Blueprint/Character/CharacterMaster.InteractWith` _ascharacter_master)))
      (else
        (bind _ascharacter_master_2 (`/Game/Blueprint/FL_Main.Get Player Character Master`))
        (`/Engine/EditorBlueprintResources/StandardMacros.IsValid` _ascharacter_master_2
          (:`Is Valid`
            (`/Game/Blueprint/Character/CharacterMaster.InteractWithEnnemy` _ascharacter_master_2))))))
  (:`Released`
    (if (not (`self.IsBeingAttack`))
      (bind _ascharacter_master_3 (`/Game/Blueprint/FL_Main.Get Player Character Master`))
      (`/Engine/EditorBlueprintResources/StandardMacros.IsValid` _ascharacter_master_3
        (:`Is Valid`
          (`/Game/Blueprint/Character/CharacterMaster.StopInteracting` _ascharacter_master_3)))
      (else
        (bind _ascharacter_master_4 (`/Game/Blueprint/FL_Main.Get Player Character Master`))
        (`/Engine/EditorBlueprintResources/StandardMacros.IsValid` _ascharacter_master_4
          (:`Is Valid`
            (`/Game/Blueprint/Character/CharacterMaster.StopInteractingWithEnnemy` _ascharacter_master_4)))))))

(event `InputAxis|Vertical`
  (params (AxisValue :type "Float (single-precision)"))
  (bind _in_game_ui (`self.In Game UI`))
  (bind _in_game_ui_2 (`self.In Game UI`))
  ;[0 0 1] Movement Vertical Axis
  (if (`/Game/UI/UI_InGame/Widget_HeadUp.InQTE` (`self.In Game UI`))
    (if (> AxisValue 0.0)
      (`/Engine/EditorBlueprintResources/StandardMacros.IsValid` _in_game_ui
        (:`Is Valid`
          (`/Game/UI/UI_InGame/Widget_HeadUp.EnterInput` _in_game_ui 1)))
      (elif (< AxisValue 0.0)
        (`/Engine/EditorBlueprintResources/StandardMacros.IsValid` _in_game_ui_2
          (:`Is Valid`
            (`/Game/UI/UI_InGame/Widget_HeadUp.EnterInput` _in_game_ui_2 3)))))
    (else
      (bind _ascharacter_master (`/Game/Blueprint/FL_Main.Get Player Character Master`))
      (`/Engine/EditorBlueprintResources/StandardMacros.IsValid` _ascharacter_master
        (:`Is Valid`
          (`/Game/Blueprint/Character/CharacterMaster.VerticalMovement` _ascharacter_master AxisValue))))))

(event `InputAction|Separate`
  (params (Key :type "Key Structure"))
  ;[0 0 1] Regroup / Separate
  (:`Pressed`
    (if (not (`self.IsBeingAttack`))
      (bind _ascharacter_master (`/Game/Blueprint/FL_Main.Get Player Character Master`))
      (`/Game/Blueprint/Character/CharacterMaster.Separate` _ascharacter_master))))

(event `InputAction|ThirdSkill`
  (params (Key :type "Key Structure"))
  ;[0 0 1] Skills
  (:`Pressed`
    (if (not (`/Game/UI/UI_InGame/Widget_HeadUp.InQTE` (`self.In Game UI`)))
      (if (not (`self.IsBeingAttack`))
        (bind _ascharacter_master (`/Game/Blueprint/FL_Main.Get Player Character Master`))
        (`/Game/Blueprint/Character/CharacterMaster.ThirdSkillActivation` _ascharacter_master)))))

(event `InputAction|UseSkills`
  (params (Key :type "Key Structure"))
  ;[0 0 1] Use Skills
  (:`Pressed`
    (if (not (`/Game/UI/UI_InGame/Widget_HeadUp.InQTE` (`self.In Game UI`)))
      (if (not (`self.IsBeingAttack`))
        (bind _ascharacter_master (`/Game/Blueprint/FL_Main.Get Player Character Master`))
        (`/Game/Blueprint/Character/CharacterMaster.UsingFirstSkill` _ascharacter_master)))))

(fn `UserConstructionScript`)