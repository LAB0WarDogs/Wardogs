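; BP_SecondChara is the second playable character, a child Blueprint that gives the parent's three skill slots a pump shotgun, a squeaky toy and a grenade.
; Skill overrides call the parent, then forward to the skill objects, with only shotgun and grenade receiving use and cancel calls.
; BeginPlay binds the player character master's inventory battery event to UseBattery.
; Incoming damage routes to TakeDamageFromEnnemyOrFriend, which defers to the parent.
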(event `self.ReceiveBeginPlay`
  ;[0 0 1] Comment
  (`parent.ReceiveBeginPlay`)
  (bind _ascharacter_master (`/Game/Blueprint/FL_Main.Get Player Character Master`))
  (add `self.UseBatteryFromInventory` _ascharacter_master (delegate `UsingBattery-SecondChara`)))

(event `UsingBattery-SecondChara`
  ;[0 0 1] Comment
  (`self.UseBattery`))

(event `/Game/Blueprint/BPI_Damageable.TakeDamage`
  (params (Damage :type "Float (single-precision)"))
  ;[0 0 1] Take Damage
  (`self.TakeDamageFromEnnemyOrFriend` Damage))

(fn `ActivateFirstSkill`
  (`parent.ActivateFirstSkill`)
  (`/Game/Blueprint/SkiilsActorComponent/BP_FusilAPompe.ActivateFirstSkill` (`self.BP_FusilAPompe`)))

(fn `ActivateSecondSkill`
  (`parent.ActivateSecondSkill`)
  (`/Game/Blueprint/SkiilsActorComponent/BP_squeakyToySkill.ActivateSecondSkill` (`self.BP_squeakyToySkill`)))

(fn `ActivateThirdSkill`
  (`parent.ActivateThirdSkill`)
  (`/Game/Blueprint/SkiilsActorComponent/BP_GrenadeSkill.ActivateThirdSkill` (`self.BP_Grenade`)))

(fn `CancelSkill`
  (params (`FirstSkillActive?` :type Boolean) (`SecondSkillActive?` :type Boolean) (`ThirdSkillActive?` :type Boolean))
  (`parent.CancelSkill` `FirstSkillActive?` `SecondSkillActive?` `ThirdSkillActive?`)
  (if (`local.FirstSkillActive?`)
    (`/Game/Blueprint/SkiilsActorComponent/BP_FusilAPompe.Cancelation` (`self.BP_FusilAPompe`))
    (elif (`local.ThirdSkillActive?`)
      (`/Game/Blueprint/SkiilsActorComponent/BP_GrenadeSkill.Cancelation` (`self.BP_Grenade`)))))

(fn `GetHealth`
  (params (DamageTaken :type "Float (double-precision)"))
  (`parent.GetHealth` DamageTaken))

(fn `TakeDamageFromEnnemyOrFriend`
  (params (DamageTaken :type "Float (double-precision)"))
  (`parent.TakeDamageFromEnnemyOrFriend` DamageTaken))

(fn `UseBattery`
  (`parent.UseBattery`))

(fn `UseFirstSkill`
  (params (`FirstSkillActive?` :type Boolean) (`SecondSkillActive?` :type Boolean) (`ThirdSkillActive?` :type Boolean))
  (`parent.UseFirstSkill` `FirstSkillActive?` `SecondSkillActive?` `ThirdSkillActive?`)
  (if (`local.FirstSkillActive?`)
    (`/Game/Blueprint/SkiilsActorComponent/BP_FusilAPompe.UseFirstSkill` (`self.BP_FusilAPompe`))
    (elif (`local.ThirdSkillActive?`)
      (`/Game/Blueprint/SkiilsActorComponent/BP_GrenadeSkill.UsingThirdSkill` (`self.BP_Grenade`)))))

(fn `UserConstructionScript`
  (`parent.UserConstructionScript`))