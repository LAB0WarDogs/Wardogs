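; Playable character Blueprint for the first Wardogs character, routing its three skill slots to sniper, flair and camouflage components.
; Timelines drive camo fading through the MPC_Stealth parameter collection and spring-arm zoom for sniping.
; A grappling move lerps the actor between two points with distance-scaled duration, updating the cable on a looping timer and blocking character switching until arrival.
; An inventory battery event uses a battery only while camouflage is active.
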(event `self.ReceiveBeginPlay`
  ;[0 0 1] Comment
  (`parent.ReceiveBeginPlay`)
  (bind _ascharacter_master (`/Game/Blueprint/FL_Main.Get Player Character Master`))
  (add `self.UseBatteryFromInventory` _ascharacter_master (delegate `UseBattery-FirstChara`))
  (bind _asgame_mode_wardogs (`/Game/Blueprint/FL_Main.GetGameMode`))
  (set `self.As Game Mode Wardogs` _asgame_mode_wardogs))

(event `UseBattery-FirstChara`
  ;[0 0 1] Comment
  (if (`/Game/Blueprint/SkiilsActorComponent/BP_Camouflage.SkillIsBeingUsed?` (`self.BP_Camouflage`))
    (`self.UseBattery`)))

(event `UsingCamo`
  ;[0 0 1] Timeline Camo
  (bind (_direction _opacity _normal_depth) (`Timeline|Timeline_0_0` :!via `PlayFromStart` :!label _label)
    (:`Update`
      (`KismetMaterialLibrary.SetScalarParameterValue` "/Game/Material/Stealth/MPC_Stealth.MPC_Stealth" "Opacity" _opacity)
      (`KismetMaterialLibrary.SetScalarParameterValue` "/Game/Material/Stealth/MPC_Stealth.MPC_Stealth" "Normal Depth" _normal_depth))))

(event `/Game/Blueprint/BPI_Damageable.TakeDamage`
  (params (Damage :type "Float (single-precision)"))
  ;[0 0 1] Take Damage
  (`self.TakeDamageFromEnnemyOrFriend` Damage))

(event `StopUsingCamo`
  ;[0 0 1] Timeline Camo
  (goto _label :!via `Reverse`))

(event `Zoom`
  ;[0 0 1] Timeline Zoom Dezoom
  (`TimelineComponent.SetPlayRate` (`self.ZoomDezoomTL`) (/ 1.0 (`self.ZoomDezoomTimeSniperSkill`)))
  (bind (_direction _zoom_dezoom) (`Timeline|ZoomDezoomTL` :!label _label_2)
    (:`Update`
      (set `SpringArmComponent.TargetArmLength` (`KismetMathLibrary.Lerp` 1200.0 1600.0 _zoom_dezoom) (`self.SpringArm`)))))

(event `Dezoom`
  ;[0 0 1] Timeline Zoom Dezoom
  (goto _label_2 :!via `ReverseFromEnd`))

(event `MovePlayerAlongGrapple`
  (bind _as_game_mode_wardogs (`self.As Game Mode Wardogs`))
  (bind _as_game_mode_wardogs_2 (`self.As Game Mode Wardogs`))
  ;[0 0 1] Move the player along the grappling hook
  (`/Engine/EditorBlueprintResources/StandardMacros.IsValid` _as_game_mode_wardogs_2
    (:`Is Valid`
      (set `/Game/Blueprint/GameMode/GameModeWardogs.CanSwitch` false _as_game_mode_wardogs_2)
      (set `self.IsUsingSkill` true)
      (`SceneComponent.SetVisibility` (`self.Cable`) true false)
      (`TimelineComponent.SetPlayRate` (`self.MovePlayer`) (/ 1.0 (`KismetMathLibrary.FClamp` (/ (`KismetMathLibrary.VSize` (- (`self.GrappleEndLocation`) (`self.GrappleStartLocation`))) 1200.0) 1.0 5.0)))
      (bind _returnvalue (`KismetSystemLibrary.K2_SetTimerDelegate` (delegate `SetGrapplingHookEndLocaton`) 0.01 true))
      (`CharacterMovementComponent.DisableMovement` (`self.CharacterMovement`))
      (bind (_direction _grapplingtrack) (`Timeline|MovePlayer` :!via `PlayFromStart`)
        (:`Update`
          (`self.K2_SetActorLocation` (`KismetMathLibrary.VLerp` (`self.GrappleStartLocation`) (`self.GrappleEndLocation`) _grapplingtrack)))
        (:`Finished`
          (`CharacterMovementComponent.SetMovementMode` (`self.CharacterMovement`) "MOVE_Walking" 0)
          (`KismetSystemLibrary.K2_ClearAndInvalidateTimerHandle` _returnvalue)
          (`SceneComponent.SetVisibility` (`self.Cable`) false false)
          (set `self.IsUsingSkill` false)
          (`/Engine/EditorBlueprintResources/StandardMacros.IsValid` _as_game_mode_wardogs
            (:`Is Valid`
              (set `/Game/Blueprint/GameMode/GameModeWardogs.CanSwitch` true _as_game_mode_wardogs))))))))

(event `SetGrapplingHookEndLocaton`
  ;[0 0 1] Move the player along the grappling hook
  (set `CableComponent.EndLocation` (`KismetMathLibrary.InverseTransformLocation` (`self.GetTransform`) (`self.GrappleEndLocation`)) (`self.Cable`)))

(fn `ActivateFirstSkill`
  (`parent.ActivateFirstSkill`)
  (`/Game/Blueprint/SkiilsActorComponent/BP_SniperSkill.ActivateSniperSkill` (`self.BP_SniperSkill`)))

(fn `ActivateSecondSkill`
  (`parent.ActivateSecondSkill`)
  (`/Game/Blueprint/SkiilsActorComponent/BP_FlairSkill.ActivateSecondSkill` (`self.BP_FlairSkill`)))

(fn `ActivateThirdSkill`
  (`parent.ActivateThirdSkill`)
  (`/Game/Blueprint/SkiilsActorComponent/BP_Camouflage.ActivateThirdSkill` (`self.BP_Camouflage`)))

(fn `CancelSkill`
  (params (`FirstSkillActive?` :type Boolean) (`SecondSkillActive?` :type Boolean) (`ThirdSkillActive?` :type Boolean))
  (`parent.CancelSkill` `FirstSkillActive?` `SecondSkillActive?` `ThirdSkillActive?`)
  (if (`local.FirstSkillActive?`)
    (`/Game/Blueprint/SkiilsActorComponent/BP_SniperSkill.Cancelation` (`self.BP_SniperSkill`))
    (elif (`local.SecondSkillActive?`)
      _
      (elif (`local.ThirdSkillActive?`)
        (`/Game/Blueprint/SkiilsActorComponent/BP_Camouflage.Cancelation` (`self.BP_Camouflage`))))))

(fn `GetHealth`
  (params (DamageTaken :type "Float (double-precision)"))
  (`parent.GetHealth` DamageTaken))

(fn `TakeDamageFromEnnemyOrFriend`
  (params (DamageTaken :type "Float (double-precision)"))
  (`parent.TakeDamageFromEnnemyOrFriend` DamageTaken))

(fn `UseBattery`
  (`parent.UseBattery`))

(fn `UseFirstSkill`
  (params (`FirstSkillActive?` :type Boolean) (`SecondSkillActive?` :type Boolean) (`ThirdSkillActive?` :type Boolean))
  (`parent.UseFirstSkill` `FirstSkillActive?` `SecondSkillActive?` `ThirdSkillActive?`)
  (if (`local.FirstSkillActive?`)
    (`/Game/Blueprint/SkiilsActorComponent/BP_SniperSkill.UseSniperSkill` (`self.BP_SniperSkill`))))

(fn `UserConstructionScript`
  (`parent.UserConstructionScript`))